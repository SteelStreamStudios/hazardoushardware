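; Electrical breaker switch that the player throws once to trigger a scripted power-up cutscene, chosen by its Switch enum.
; Box overlap by the player scales a prompt plane in and out.
; PowerOn disables input, flips the handle with sparks, then uses delay-chained camera blends and, in most variants, level sequences before restoring control.
; Variants drive flame hazard and fence door, assembly arms and conveyors, machine turrets, or just the fence door.
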(event `self.ReceiveBeginPlay`
  (bind _asbp_game_state (cast `/Game/Blueprints/Class/BP_GameState` (`GameplayStatics.GetGameState`)))
  (set `self.As BP Game State` _asbp_game_state)
  (bind _asbp_robot (cast `/Game/Blueprints/Class/BP_Robot` (`GameplayStatics.GetPlayerPawn` 0)))
  (set `self.As BP Robot` _asbp_robot))

(event `self.Box.OnComponentBeginOverlap`
  (params (OverlappedComponent :type "PrimitiveComponent Object Reference") (OtherActor :type "Actor Object Reference") (OtherComp :type "PrimitiveComponent Object Reference") (OtherBodyIndex :type Integer) (bFromSweep :type Boolean) (SweepResult :type "HitResult Structure (by ref)"))
  (if (== OtherActor (`GameplayStatics.GetPlayerPawn` 0))
    (`self.UIOn`)))

(event `self.Box.OnComponentEndOverlap`
  (params (OverlappedComponent :type "PrimitiveComponent Object Reference") (OtherActor :type "Actor Object Reference") (OtherComp :type "PrimitiveComponent Object Reference") (OtherBodyIndex :type Integer))
  (if (== OtherActor (`GameplayStatics.GetPlayerPawn` 0))
    (`self.UIOff`)))

(event `UIOn`
  (`/Engine/EditorBlueprintResources/StandardMacros.DoOnce` false :!label _label
    (:`Completed`
      (`|ExecutionSequence`
        (:`then_0`
          (bind (_direction _newtrack_0) (`Timeline|Timeline` :!via `Stop` :!label _label_2)
            (:`Update`
              (`SceneComponent.SetWorldScale3D` (`self.Plane`) (`KismetMathLibrary.VLerp` (2.0 2.0 2.0) (0.0 0.0 0.0) _newtrack_0)))
            (:`Finished`
              (goto _label :!via `Reset`))))
        (:`then_1`
          (bind (_direction_2 _newtrack_0_2) (`Timeline|On` :!via `PlayFromStart` :!label _label_3)
            (:`Update`
              (`SceneComponent.SetWorldScale3D` (`self.Plane`) (`KismetMathLibrary.VLerp` (0.0 0.0 0.0) (2.0 2.0 2.0) _newtrack_0_2)))
            (:`Finished`
              (goto _label_4 :!via `Reset`))))))))

(event `UIOff`
  (`/Engine/EditorBlueprintResources/StandardMacros.DoOnce` false :!label _label_4
    (:`Completed`
      (`|ExecutionSequence`
        (:`then_0`
          (goto _label_3 :!via `Stop`))
        (:`then_1`
          (goto _label_2 :!via `PlayFromStart`))))))

(event `PowerOn`
  (bind _returnvalue (`GameplayStatics.GetPlayerController` 0))
  (bind _returnvalue_2 (`GameplayStatics.GetPlayerController` 0))
  (bind _arrow (`self.Arrow`))
  (bind _arrow_2 (`self.Arrow`))
  (bind _arrow_3 (`self.Arrow`))
  (bind _arrow_4 (`self.Arrow`))
  (bind _returnvalue_3 (`SceneComponent.K2_GetComponentLocation` (`self.Handle`)))
  (if (`|EnumEquality` (`self.Switch`) "NewEnumerator0")
    (`/Engine/EditorBlueprintResources/StandardMacros.DoOnce` false
      (:`Completed`
        (`self.DisableInput` (`GameplayStatics.GetPlayerPawn` 0) _returnvalue_2)
        (bind _asbp_player_controller (cast `/Game/Blueprints/Class/BP_PlayerController` _returnvalue_2))
        (bind _output_get (set `self.As BP Player Controller` _asbp_player_controller))
        (set `/Game/Blueprints/Class/BP_PlayerController.CanRotate` false _output_get)
        (`SceneComponent.SetVisibility` (`self.Plane`) false false)
        (`|ExecutionSequence`
          (:`then_0`
            (bind (_direction _time) (`Timeline|SwitchUp` :!via `PlayFromStart`)
              (:`Update`
                (`SceneComponent.K2_SetRelativeRotation` (`self.Handle`) (`KismetMathLibrary.RLerp` (struct :`Roll` 180.0) (struct) _time) false false))
              (:`Finished`
                (`NiagaraFunctionLibrary.SpawnSystemAtLocation` "/Game/VFX/PS_Sparks.PS_Sparks" (`SceneComponent.K2_GetComponentLocation` _arrow) (`SceneComponent.K2_GetComponentRotation` _arrow))
                (`KismetSystemLibrary.Delay` 0.8)
                (bind _returnvalue_4 (`GameplayStatics.GetActorOfClass` "/Game/Blueprints/Class/BP_Camera.BP_Camera_C"))
                (`PlayerController.SetViewTargetWithBlend` (`GameplayStatics.GetPlayerController` 0) _returnvalue_4 3.0 "VTBlend_Linear" 0.0 false)
                (`KismetSystemLibrary.Delay` 1.5)
                (`/Game/Blueprints/Class/BP_Robot.EarsOnCamera` (`self.As BP Robot`))
                (`KismetSystemLibrary.Delay` 1.5)
                (set `self.PoweredOn` true)
                (`KismetSystemLibrary.Delay` 3.2)
                (bind _returnvalue_5 (`GameplayStatics.GetActorOfClass` "/Game/Blueprints/Class/BP_Camera2.BP_Camera2_C"))
                (`PlayerController.SetViewTargetWithBlend` _returnvalue _returnvalue_5 2.0 "VTBlend_Linear" 0.0 false)
                (`KismetSystemLibrary.Delay` 3.0)
                (`PlayerController.SetAudioListenerOverride` :`self` _returnvalue :`AttachToComponent` (`/Game/Blueprints/Class/BP_Camera2.CineCamera` _returnvalue_5))
                (bind _returnvalue_6 (`GameplayStatics.GetActorOfClass` "/Game/Blueprints/Class/BP_FlameHazard.BP_FlameHazard_C"))
                (`/Game/Blueprints/Class/BP_FlameHazard.TurnOn` _returnvalue_6)
                (`KismetSystemLibrary.Delay` 0.5)
                (bind (_outactor _returnvalue_7) (`LevelSequencePlayer.CreateLevelSequencePlayer` "/Game/Sequences/MeltRailing.MeltRailing"))
                (`MovieSceneSequencePlayer.Play` _returnvalue_7)
                (bind _returnvalue_8 (`GameplayStatics.GetActorOfClass` "/Game/Blueprints/Class/BP_Camera.BP_Camera_C"))
                (`/Game/Blueprints/Class/BP_Camera.Move1` _returnvalue_8)
                (`PlayerController.SetAudioListenerOverride` :`self` (`GameplayStatics.GetPlayerController` 0) :`AttachToComponent` (`/Game/Blueprints/Class/BP_Camera.CineCamera` _returnvalue_8))
                (`KismetSystemLibrary.Delay` 5.0)
                (`PlayerController.SetViewTargetWithBlend` (`GameplayStatics.GetPlayerController` 0) _returnvalue_8 3.0 "VTBlend_Linear" 0.0 false)
                (`KismetSystemLibrary.Delay` 3.2)
                (bind _returnvalue_9 (`GameplayStatics.GetActorOfClass` "/Game/Blueprints/Class/BP_FenceDoor.BP_FenceDoor_C"))
                (`/Game/Blueprints/Class/BP_FenceDoor.OpenDoor` _returnvalue_9)
                (`KismetSystemLibrary.Delay` 2.0)
                (`PlayerController.SetViewTargetWithBlend` (`GameplayStatics.GetPlayerController` 0) (`GameplayStatics.GetPlayerPawn` 0) 2.0 "VTBlend_Linear" 0.0 false)
                (`KismetSystemLibrary.Delay` 1.0)
                (`/Game/Blueprints/Class/BP_Robot.EarsOnMesh` (`self.As BP Robot`))
                (`KismetSystemLibrary.Delay` 1.0)
                (`/Game/Blueprints/Class/BP_Robot.ResetMousePosition` (`self.As BP Robot`))
                (set `/Game/Blueprints/Class/BP_PlayerController.CanRotate` true (`self.As BP Player Controller`))
                (`self.EnableInput` (`GameplayStatics.GetPlayerPawn` 0) (`GameplayStatics.GetPlayerController` 0))
                (bind _returnvalue_10 (`GameplayStatics.GetActorOfClass` "/Game/Blueprints/Class/BP_Camera.BP_Camera_C"))
                (`/Game/Blueprints/Class/BP_Camera.Move2` _returnvalue_10))))
          (:`then_1`
            (`KismetSystemLibrary.Delay` 1.0)
            (`GameplayStatics.PlaySoundAtLocation` "/Game/Audio/Level1/Breaker-Switch.Breaker-Switch" _returnvalue_3 (struct) 1.0 1.0 0.0 "/Game/Audio/FurnaceSoundAttenuation.FurnaceSoundAttenuation" null null null)
            (`GameplayStatics.PlaySoundAtLocation` "/Game/Audio/Level1/Electrical__Spark_High_voltage.Electrical__Spark_High_voltage" _returnvalue_3 (struct) 1.0 1.0 0.0 "/Game/Audio/FurnaceSoundAttenuation.FurnaceSoundAttenuation" null null null)))))
    (elif (`|EnumEquality` (`self.Switch`) "NewEnumerator1")
      (`/Engine/EditorBlueprintResources/StandardMacros.DoOnce` false
        (:`Completed`
          (`self.DisableInput` (`GameplayStatics.GetPlayerPawn` 0) (`GameplayStatics.GetPlayerController` 0))
          (`SceneComponent.SetVisibility` (`self.Plane`) false false)
          (bind (_direction_2 _time_2) (`Timeline|Timeline_0` :!via `PlayFromStart`)
            (:`Update`
              (`SceneComponent.K2_SetRelativeRotation` (`self.Handle`) (`KismetMathLibrary.RLerp` (struct :`Roll` 180.0) (struct) _time_2) false false))
            (:`Finished`
              (`NiagaraFunctionLibrary.SpawnSystemAtLocation` "/Game/VFX/PS_Sparks.PS_Sparks" (`SceneComponent.K2_GetComponentLocation` _arrow_4) (`SceneComponent.K2_GetComponentRotation` _arrow_4))
              (`KismetSystemLibrary.Delay` 0.8)
              (bind _returnvalue_11 (`GameplayStatics.GetActorOfClass` "/Game/Blueprints/Class/BP_Camera.BP_Camera_C"))
              (`PlayerController.SetViewTargetWithBlend` (`GameplayStatics.GetPlayerController` 0) _returnvalue_11 3.0 "VTBlend_Linear" 0.0 false)
              (`KismetSystemLibrary.Delay` 3.0)
              (bind (_outactor_2 _returnvalue_12) (`LevelSequencePlayer.CreateLevelSequencePlayer` "/Game/Sequences/Level2PowerUp.Level2PowerUp"))
              (`MovieSceneSequencePlayer.Play` _returnvalue_12)
              (`KismetSystemLibrary.Delay` 0.5)
              (set `self.PoweredOn` true)
              (`self.TurnOnArms`
                (:`Completed`
                  (`self.TurnOnConveyor`
                    (:`Completed`
                      (`KismetSystemLibrary.Delay` 17.0)
                      (`PlayerController.SetViewTargetWithBlend` (`GameplayStatics.GetPlayerController` 0) (`GameplayStatics.GetPlayerPawn` 0) 2.0 "VTBlend_Linear" 0.0 false)
                      (`KismetSystemLibrary.Delay` 2.0)
                      (`self.EnableInput` (`GameplayStatics.GetPlayerPawn` 0) (`GameplayStatics.GetPlayerController` 0))))))))))
      (elif (`|EnumEquality` (`self.Switch`) "NewEnumerator2")
        (`/Engine/EditorBlueprintResources/StandardMacros.DoOnce` false
          (:`Completed`
            (`self.DisableInput` (`GameplayStatics.GetPlayerPawn` 0) (`GameplayStatics.GetPlayerController` 0))
            (`SceneComponent.SetVisibility` (`self.Plane`) false false)
            (bind (_direction_3 _time_3) (`Timeline|Timeline_1` :!via `PlayFromStart`)
              (:`Update`
                (`SceneComponent.K2_SetRelativeRotation` (`self.Handle`) (`KismetMathLibrary.RLerp` (struct :`Roll` 180.0) (struct) _time_3) false false))
              (:`Finished`
                (`NiagaraFunctionLibrary.SpawnSystemAtLocation` "/Game/VFX/PS_Sparks.PS_Sparks" (`SceneComponent.K2_GetComponentLocation` _arrow_2) (`SceneComponent.K2_GetComponentRotation` _arrow_2))
                (`KismetSystemLibrary.Delay` 0.8)
                (bind _returnvalue_13 (`GameplayStatics.GetActorOfClass` "/Game/Blueprints/Class/BP_Camera2.BP_Camera2_C"))
                (`PlayerController.SetViewTargetWithBlend` (`GameplayStatics.GetPlayerController` 0) _returnvalue_13 3.0 "VTBlend_Linear" 0.0 false)
                (`KismetSystemLibrary.Delay` 3.0)
                (bind (_outactor_3 _returnvalue_14) (`LevelSequencePlayer.CreateLevelSequencePlayer` "/Game/Sequences/OpenShieldCase.OpenShieldCase"))
                (`MovieSceneSequencePlayer.Play` _returnvalue_14)
                (`KismetSystemLibrary.Delay` 3.0)
                (`|ExecutionSequence`
                  (:`then_0`
                    (bind _returnvalue_15 (`GameplayStatics.GetActorOfClass` "/Game/Blueprints/Class/BP_MachineTurret.BP_MachineTurret_C"))
                    (`/Game/Blueprints/Class/BP_MachineTurret.RaiseTurret` _returnvalue_15))
                  (:`then_1`
                    (bind _outactors (`GameplayStatics.GetAllActorsOfClass` "/Game/Blueprints/Class/BP_MachineTurret.BP_MachineTurret_C"))
                    (for _array_element _outactors
                      (`/Game/Blueprints/Class/BP_MachineTurret.PowerUp` _array_element)
                      (`/Game/Blueprints/Class/BP_MachineTurret.Fire` _array_element))
                    (`KismetSystemLibrary.Delay` 0.15)
                    (`PlayerController.SetViewTargetWithBlend` (`GameplayStatics.GetPlayerController` 0) (`GameplayStatics.GetPlayerPawn` 0) 0.0 "VTBlend_Linear" 0.0 false)
                    (`self.EnableInput` (`GameplayStatics.GetPlayerPawn` 0) (`GameplayStatics.GetPlayerController` 0))))))))
        (elif (`|EnumEquality` (`self.Switch`) "NewEnumerator3")
          (`/Engine/EditorBlueprintResources/StandardMacros.DoOnce` false
            (:`Completed`
              (`self.DisableInput` (`GameplayStatics.GetPlayerPawn` 0) (`GameplayStatics.GetPlayerController` 0))
              (`SceneComponent.SetVisibility` (`self.Plane`) false false)
              (bind (_direction_4 _time_4) (`Timeline|Timeline_2` :!via `PlayFromStart`)
                (:`Update`
                  (`SceneComponent.K2_SetRelativeRotation` (`self.Handle`) (`KismetMathLibrary.RLerp` (struct :`Roll` 180.0) (struct) _time_4) false false))
                (:`Finished`
                  (`NiagaraFunctionLibrary.SpawnSystemAtLocation` "/Game/VFX/PS_Sparks.PS_Sparks" (`SceneComponent.K2_GetComponentLocation` _arrow_3) (`SceneComponent.K2_GetComponentRotation` _arrow_3))
                  (`KismetSystemLibrary.Delay` 0.8)
                  (bind _returnvalue_16 (`GameplayStatics.GetActorOfClass` "/Game/Blueprints/Class/BP_Camera.BP_Camera_C"))
                  (`PlayerController.SetViewTargetWithBlend` (`GameplayStatics.GetPlayerController` 0) _returnvalue_16 3.0 "VTBlend_EaseInOut" 2.0 false)
                  (`KismetSystemLibrary.Delay` 3.0)
                  (bind _returnvalue_17 (`GameplayStatics.GetActorOfClass` "/Game/Blueprints/Class/BP_FenceDoor.BP_FenceDoor_C"))
                  (`/Game/Blueprints/Class/BP_FenceDoor.OpenDoor` _returnvalue_17)
                  (`KismetSystemLibrary.Delay` 3.0)
                  (`PlayerController.SetViewTargetWithBlend` (`GameplayStatics.GetPlayerController` 0) (`GameplayStatics.GetPlayerPawn` 0) 2.0 "VTBlend_EaseInOut" 2.0 false)
                  (`KismetSystemLibrary.Delay` 2.0)
                  (`self.EnableInput` (`GameplayStatics.GetPlayerPawn` 0) (`GameplayStatics.GetPlayerController` 0)))))))))))

(fn `UserConstructionScript`)