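; Inclined conveyor belt that carries BP_Robot actors along its three sections.
; BeginPlay creates dynamic materials to set the belt's glow and the tread's scroll speed, which is separate from PushSpeed.
; Tick finds the first trigger box overlapping the player pawn, then offsets every robot in it along that box's arrow, scaled by PushSpeed and delta time, without sweeping.
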(event `self.ReceiveBeginPlay`
  (bind _conveyorbelt (`self.ConveyorBelt`))
  (bind _tread (`self.Tread`))
  (bind _returnvalue (`PrimitiveComponent.CreateDynamicMaterialInstance` _conveyorbelt 0 (`PrimitiveComponent.GetMaterial` _conveyorbelt 0) "None"))
  (bind _output_get (set `self.Mat` _returnvalue))
  (`MaterialInstanceDynamic.SetScalarParameterValue` _output_get "Glow" (`self.Glow`))
  (bind _returnvalue_2 (`PrimitiveComponent.CreateDynamicMaterialInstance` _tread 0 (`PrimitiveComponent.GetMaterial` _tread 0) "None"))
  (`MaterialInstanceDynamic.SetScalarParameterValue` _returnvalue_2 "SpeedY" (`self.Speed`)))

(event `self.ReceiveTick`
  (params (DeltaSeconds :type "Float (single-precision)"))
  (if (`PrimitiveComponent.IsOverlappingActor` (`self.Box`) (`GameplayStatics.GetPlayerPawn` 0))
    (for _array_element (`PrimitiveComponent.GetOverlappingActors` (`self.Box`) "/Game/Blueprints/Class/BP_Robot.BP_Robot_C")
      (`self.K2_AddActorWorldOffset` _array_element (* (`KismetMathLibrary.GetForwardVector` (`SceneComponent.K2_GetComponentRotation` (`self.Arrow`))) (* DeltaSeconds (`self.PushSpeed`))) false false))
    (elif (`PrimitiveComponent.IsOverlappingActor` (`self.Box1`) (`GameplayStatics.GetPlayerPawn` 0))
      (for _array_element_2 (`PrimitiveComponent.GetOverlappingActors` (`self.Box1`) "/Game/Blueprints/Class/BP_Robot.BP_Robot_C")
        (`self.K2_AddActorWorldOffset` _array_element_2 (* (`KismetMathLibrary.GetForwardVector` (`SceneComponent.K2_GetComponentRotation` (`self.Arrow1`))) (* DeltaSeconds (`self.PushSpeed`))) false false))
      (elif (`PrimitiveComponent.IsOverlappingActor` (`self.Box2`) (`GameplayStatics.GetPlayerPawn` 0))
        (for _array_element_3 (`PrimitiveComponent.GetOverlappingActors` (`self.Box2`) "/Game/Blueprints/Class/BP_Robot.BP_Robot_C")
          (`self.K2_AddActorWorldOffset` _array_element_3 (* (`KismetMathLibrary.GetForwardVector` (`SceneComponent.K2_GetComponentRotation` (`self.Arrow2`))) (* DeltaSeconds (`self.PushSpeed`))) false false))))))

(fn `UserConstructionScript`)