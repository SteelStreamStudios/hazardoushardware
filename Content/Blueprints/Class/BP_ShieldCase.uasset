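; BP_ShieldCase is a display case whose shield can be switched off.
; On BeginPlay it creates dynamic material instances for the display box mesh (the shield) and the sphere (the light).
; The ShieldShutOff event turns the light green and plays a timeline that fades the shield's opacity to zero.
; The shield's collision is disabled from the timeline's update, so it stops blocking as the fade starts.
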(event `self.ReceiveBeginPlay`
  (bind _sm_display_box_low_object001 (`self.SM_Display_Box_low_Object001`))
  (bind _sphere (`self.Sphere`))
  (bind _returnvalue (`PrimitiveComponent.CreateDynamicMaterialInstance` _sm_display_box_low_object001 0 (`PrimitiveComponent.GetMaterial` _sm_display_box_low_object001 0) "None"))
  (set `self.ShieldMat` _returnvalue)
  (bind _returnvalue_2 (`PrimitiveComponent.CreateDynamicMaterialInstance` _sphere 0 (`PrimitiveComponent.GetMaterial` _sphere 0) "None"))
  (set `self.LightMat` _returnvalue_2))

(event `ShieldShutOff`
  (`MaterialInstanceDynamic.SetVectorParameterValue` (`self.LightMat`) "Color" (struct :`R` 0.08194 :`G` 1.0 :`A` 1.0))
  (bind (_direction _newtrack_0) (`Timeline|Timeline` :!via `PlayFromStart`)
    (:`Update`
      (`MaterialInstanceDynamic.SetScalarParameterValue` (`self.ShieldMat`) "Opacity" (`KismetMathLibrary.Lerp` 1.0 0.0 _newtrack_0))
      (`PrimitiveComponent.SetCollisionEnabled` (`self.SM_Display_Box_low_Object001`) "NoCollision"))))

(fn `UserConstructionScript`)