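; Robotic assembly arm that can be stunned or glitched and that reacts to explosive barrels.
; Box overlap with a barrel triggers a glitch, Sphere overlap detonates the barrel, and stunning requires power; both states temporarily change color and animation.
; A duplicate skeletal mesh built in construction mirrors the animations and provides an outline through dynamic material width.
; Tick hides the outline whenever the player robot's ArmHit is unset.
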(event `self.ReceiveTick`
  (params (DeltaSeconds :type "Float (single-precision)"))
  (bind _asbp_robot (cast `/Game/Blueprints/Class/BP_Robot` (`GameplayStatics.GetPlayerPawn` 0)))
  (if (not (`/Game/Blueprints/Class/BP_Robot.ArmHit` _asbp_robot))
    (`self.RemoveOutline`)))

(event `self.ReceiveBeginPlay`
  (bind _arm (`self.Arm`))
  (bind _addskeletalmesh (`self.AddSkeletalMesh`))
  (for (_array_element _array_index) (`MeshComponent.GetMaterials` _arm)
    (bind _returnvalue (`PrimitiveComponent.CreateDynamicMaterialInstance` _arm _array_index _array_element "None"))
    (`KismetArrayLibrary.Array_Set` (`self.Target Array`) _array_index _returnvalue true))
  (for (_array_element_2 _array_index_2) (`MeshComponent.GetMaterials` _addskeletalmesh)
    (bind _returnvalue_2 (`PrimitiveComponent.CreateDynamicMaterialInstance` _addskeletalmesh _array_index_2 _array_element_2 "None"))
    (`KismetArrayLibrary.Array_Set` (`self.OutlineArray`) _array_index_2 _returnvalue_2 true))
  (`self.SetValues`))

(event `SetValues`
  (for _array_element (`self.Target Array`)
    (`MaterialInstanceDynamic.SetScalarParameterValue` _array_element "Glow" (`self.Glow`))
    (`MaterialInstanceDynamic.SetVectorParameterValue` _array_element "Color" (`self.Color`)))
  (for _array_element_2 (`self.OutlineArray`)
    (`MaterialInstanceDynamic.SetScalarParameterValue` _array_element_2 "Width" (`self.Width`))))

(event `self.Box.OnComponentBeginOverlap`
  (params (OverlappedComponent :type "PrimitiveComponent Object Reference") (OtherActor :type "Actor Object Reference") (OtherComp :type "PrimitiveComponent Object Reference") (OtherBodyIndex :type Integer) (bFromSweep :type Boolean) (SweepResult :type "HitResult Structure (by ref)"))
  (cast `/Game/Blueprints/Class/BP_ExplosiveBarrel` OtherActor)
  (`self.Glitch`))

(event `self.Sphere.OnComponentBeginOverlap`
  (params (OverlappedComponent :type "PrimitiveComponent Object Reference") (OtherActor :type "Actor Object Reference") (OtherComp :type "PrimitiveComponent Object Reference") (OtherBodyIndex :type Integer) (bFromSweep :type Boolean) (SweepResult :type "HitResult Structure (by ref)"))
  (bind _asbp_explosive_barrel (cast `/Game/Blueprints/Class/BP_ExplosiveBarrel` OtherActor))
  (`/Game/Blueprints/Class/BP_ExplosiveBarrel.Explode` _asbp_explosive_barrel))

(event `Stun`
  (if (`self.PoweredOn`)
    (if (not (`self.Stunned`))
      (set `self.Stunned` true)
      (set `self.Color` (struct :`R` 1.0 :`A` 1.0))
      (`self.SetValues`)
      (`SkeletalMeshComponent.PlayAnimation` (`self.Arm`) "/Game/Animations/Props/A_Stunned.A_Stunned" false)
      (`SkeletalMeshComponent.PlayAnimation` (`self.AddSkeletalMesh`) "/Game/Animations/Props/A_Stunned.A_Stunned" false)
      (`KismetSystemLibrary.Delay` 3.0)
      (set `self.Stunned` false)
      (set `self.Color` (struct :`G` 1.0 :`B` 0.061246 :`A` 1.0))
      (`self.SetValues`))))

(event `Glitch`
  (if (not (`self.Stunned`))
    (set `self.Color` (struct :`R` 1.0 :`G` 0.852999 :`A` 1.0))
    (`self.SetValues`)
    (`SkeletalMeshComponent.PlayAnimation` (`self.Arm`) "/Game/Animations/Props/A_Glitch.A_Glitch" false)
    (`SkeletalMeshComponent.PlayAnimation` (`self.AddSkeletalMesh`) "/Game/Animations/Props/A_Glitch.A_Glitch" false)
    (`KismetSystemLibrary.Delay` 3.2)
    (set `self.Color` (struct :`G` 1.0 :`B` 0.061246 :`A` 1.0))
    (`self.SetValues`)))

(event `AddOutline`
  (set `self.Width` 1.0)
  (`self.SetValues`))

(event `RemoveOutline`
  (set `self.Width` 0.0)
  (`self.SetValues`))

(fn `UserConstructionScript`
  (bind _arm (`self.Arm`))
  (bind _addskeletalmesh (`self.AddSkeletalMesh`))
  (bind _addskeletalmesh_2 (`self.AddSkeletalMesh`))
  (bind _returnvalue (`AddComponent|NODE_AddSkeletalMeshComponent-0` :`RelativeTransform` (`SceneComponent.GetRelativeTransform` _arm)))
  (bind _output_get (set `self.AddSkeletalMesh` _returnvalue))
  (`SkeletalMeshComponent.SetSkeletalMeshAsset` _output_get (`SkeletalMeshComponent.SkeletalMeshAsset` _arm))
  (`PrimitiveComponent.SetMaterial` _addskeletalmesh 0 "/Game/Materials/M_Outline_Inst.M_Outline_Inst")
  (`PrimitiveComponent.SetMaterial` _addskeletalmesh 1 "/Game/Materials/M_Outline_Inst.M_Outline_Inst")
  (for (_array_element _array_index) (`MeshComponent.GetMaterials` _addskeletalmesh_2)
    (bind _returnvalue_2 (`PrimitiveComponent.CreateDynamicMaterialInstance` _addskeletalmesh_2 _array_index _array_element "None"))
    (`KismetArrayLibrary.Array_Set` (`self.OutlineArray`) _array_index _returnvalue_2 true)))