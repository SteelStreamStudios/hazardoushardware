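; BP_PlasmaProjectile is a projectile that breaks destructible objects on impact.
; When its sphere component hits a BP_Destructible, it enables collision damage on that actor's geometry collection and calls its Remove function.
; It then applies an impulse scaled from its own velocity to the hit component at the sphere's location.
; The projectile destroys itself after any hit, whether or not the target is destructible.
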(event `self.Sphere.OnComponentHit`
  (params (HitComponent :type "PrimitiveComponent Object Reference") (OtherActor :type "Actor Object Reference") (OtherComp :type "PrimitiveComponent Object Reference") (NormalImpulse :type "Vector Structure") (Hit :type "HitResult Structure (by ref)"))
  (`|ExecutionSequence`
    (:`then_0`
      (bind _asbp_destructible (cast `/Game/Blueprints/Class/BP_Destructible` OtherActor))
      (`GeometryCollectionComponent.SetEnableDamageFromCollision` (`/Game/Blueprints/Class/BP_Destructible.Cube_GeometryCollection` _asbp_destructible) true)
      (`/Game/Blueprints/Class/BP_Destructible.Remove` _asbp_destructible)
      (`PrimitiveComponent.AddImpulseAtLocation` OtherComp (* (`self.GetVelocity`) 50.0) (`SceneComponent.K2_GetComponentLocation` (`self.Sphere`)) "None"))
    (:`then_1`
      (`self.K2_DestroyActor`))))

(fn `UserConstructionScript`)