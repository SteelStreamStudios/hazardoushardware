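; Elevator actor that serves as the transition between levels, cycling through three levels and back to the first.
; On BeginPlay it caches BP_GameState and plays the door-open animation if Open is set.
; When the player overlaps Box, it branches on the game state's Level, closes every BP_ElevatorDoor, waits, then plays that level's sequence and disables input.
; Sequence-finished callbacks open the next map; only the first level's branch uses DoOnce and reveals two planes.
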(event `self.ReceiveBeginPlay`
  (bind _asbp_game_state (cast `/Game/Blueprints/Class/BP_GameState` (`GameplayStatics.GetGameState`)))
  (set `self.As BP Game State` _asbp_game_state)
  (if (`self.Open?`)
    (`SkeletalMeshComponent.PlayAnimation` (`self.Door1`) "/Game/Meshes/Environment/A_ElevatorDoorOpen_Anim.A_ElevatorDoorOpen_Anim" false)))

(event `self.Box.OnComponentBeginOverlap`
  (params (OverlappedComponent :type "PrimitiveComponent Object Reference") (OtherActor :type "Actor Object Reference") (OtherComp :type "PrimitiveComponent Object Reference") (OtherBodyIndex :type Integer) (bFromSweep :type Boolean) (SweepResult :type "HitResult Structure (by ref)"))
  (if (== OtherActor (`GameplayStatics.GetPlayerPawn` 0))
    (if (`|EnumEquality` (`/Game/Blueprints/Class/BP_GameState.Level` (`self.As BP Game State`)) "NewEnumerator0")
      (`/Engine/EditorBlueprintResources/StandardMacros.DoOnce` false
        (:`Completed`
          (bind _outactors (`GameplayStatics.GetAllActorsOfClass` "/Game/Blueprints/Class/BP_ElevatorDoor.BP_ElevatorDoor_C"))
          (for _array_element _outactors
            (`/Game/Blueprints/Class/BP_ElevatorDoor.CloseDoor` _array_element))
          (`KismetSystemLibrary.Delay` 3.0)
          (`SceneComponent.SetVisibility` (`self.Plane`) true false)
          (`SceneComponent.SetVisibility` (`self.Plane1`) true false)
          (bind (_outactor _returnvalue) (`LevelSequencePlayer.CreateLevelSequencePlayer` "/Game/Sequences/ElevatorUp.ElevatorUp"))
          (`MovieSceneSequencePlayer.Play` _returnvalue)
          (add `MovieSceneSequencePlayer.OnFinished` _returnvalue (delegate `OnFinished_Event`))
          (`self.DisableInput` (`GameplayStatics.GetPlayerPawn` 0) (`GameplayStatics.GetPlayerController` 0))))
      (elif (`|EnumEquality` (`/Game/Blueprints/Class/BP_GameState.Level` (`self.As BP Game State`)) "NewEnumerator1")
        (bind _outactors_2 (`GameplayStatics.GetAllActorsOfClass` "/Game/Blueprints/Class/BP_ElevatorDoor.BP_ElevatorDoor_C"))
        (for _array_element_2 _outactors_2
          (`/Game/Blueprints/Class/BP_ElevatorDoor.CloseDoor` _array_element_2))
        (`KismetSystemLibrary.Delay` 3.0)
        (bind (_outactor_2 _returnvalue_2) (`LevelSequencePlayer.CreateLevelSequencePlayer` "/Game/Sequences/Level2ElevatorUp.Level2ElevatorUp"))
        (`MovieSceneSequencePlayer.Play` _returnvalue_2)
        (add `MovieSceneSequencePlayer.OnFinished` _returnvalue_2 (delegate `LoadLevel3`))
        (`self.DisableInput` (`GameplayStatics.GetPlayerPawn` 0) (`GameplayStatics.GetPlayerController` 0))
        (elif (`|EnumEquality` (`/Game/Blueprints/Class/BP_GameState.Level` (`self.As BP Game State`)) "NewEnumerator2")
          (bind _outactors_3 (`GameplayStatics.GetAllActorsOfClass` "/Game/Blueprints/Class/BP_ElevatorDoor.BP_ElevatorDoor_C"))
          (for _array_element_3 _outactors_3
            (`/Game/Blueprints/Class/BP_ElevatorDoor.CloseDoor` _array_element_3))
          (`KismetSystemLibrary.Delay` 3.0)
          (bind (_outactor_3 _returnvalue_3) (`LevelSequencePlayer.CreateLevelSequencePlayer` "/Game/Sequences/Level3ElevatorUp.Level3ElevatorUp"))
          (`MovieSceneSequencePlayer.Play` _returnvalue_3)
          (add `MovieSceneSequencePlayer.OnFinished` _returnvalue_3 (delegate `LoadLevel1`))
          (`self.DisableInput` (`GameplayStatics.GetPlayerPawn` 0) (`GameplayStatics.GetPlayerController` 0)))))))

(event `OnFinished_Event`
  (if (`|EnumEquality` (`/Game/Blueprints/Class/BP_GameState.Level` (`self.As BP Game State`)) "NewEnumerator0")
    (`GameplayStatics.OpenLevel` "Level2_TestingRoom")))

(event `LoadLevel3`
  (if (`|EnumEquality` (`/Game/Blueprints/Class/BP_GameState.Level` (`self.As BP Game State`)) "NewEnumerator1")
    (`GameplayStatics.OpenLevel` "Level3_StorageArea")))

(event `LoadLevel1`
  (if (`|EnumEquality` (`/Game/Blueprints/Class/BP_GameState.Level` (`self.As BP Game State`)) "NewEnumerator2")
    (`GameplayStatics.OpenLevel` "Level1_Incinerator")))

(fn `UserConstructionScript`)