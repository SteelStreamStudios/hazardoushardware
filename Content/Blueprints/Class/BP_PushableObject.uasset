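; Pushable block that the player robot shoves in fixed-distance steps, limited to the world +X direction.
; A head-on hit snaps the push direction to an axis, then disables movement, widens the capsule and attaches the player.
; A timeline slides the block with sparks, repeating while WASD is held.
; CanPush gates each step with traces for facing, clearance and floor, plus falling and equipped-gun checks.
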(event `self.ReceiveBeginPlay`
  (bind _asbp_robot (cast `/Game/Blueprints/Class/BP_Robot` (`GameplayStatics.GetPlayerPawn` 0)))
  (set `self.As BP Robot` _asbp_robot))

(event `self.ReceiveHit`
  (params (MyComp :type "PrimitiveComponent Object Reference") (Other :type "Actor Object Reference") (OtherComp :type "PrimitiveComponent Object Reference") (bSelfMoved :type Boolean) (HitLocation :type "Vector Structure") (HitNormal :type "Vector Structure") (NormalImpulse :type "Vector Structure") (Hit :type "HitResult Structure (by ref)"))
  (bind _returnvalue (`self.GetActorForwardVector` Other))
  (bind _returnvalue_2 (`GameplayStatics.GetPlayerCharacter` 0))
  (bind _capsulecomponent (`Character.CapsuleComponent` _returnvalue_2))
  (if (== (`GameplayStatics.GetPlayerPawn` 0) Other)
    (if (> (`KismetMathLibrary.Dot_VectorVector` HitNormal _returnvalue) 0.93)
      (bind _output_get (set `self.PushableDirection` (`KismetMathLibrary.MakeVector` (`KismetMathLibrary.Conv_IntToDouble` (`KismetMathLibrary.Round` (.x _returnvalue))) (`KismetMathLibrary.Conv_IntToDouble` (`KismetMathLibrary.Round` (.y _returnvalue))) (`KismetMathLibrary.Conv_IntToDouble` (`KismetMathLibrary.Round` (.z _returnvalue))))))
      (if (and (== (.y _output_get) 0.0) (> (.x _output_get) 0.0))
        (bind _canpush (`self.CanPush`))
        (if _canpush
          (`CharacterMovementComponent.DisableMovement` (`Character.CharacterMovement` _returnvalue_2))
          (`CapsuleComponent.SetCapsuleRadius` _capsulecomponent 65.0 true)
          (`KismetSystemLibrary.MoveComponentTo` _capsulecomponent (+ (`SceneComponent.K2_GetComponentLocation` _capsulecomponent) (* (`self.GetActorForwardVector` _returnvalue_2) (0.0 0.0 0.0))) (`SceneComponent.K2_GetComponentRotation` _capsulecomponent))
          (`self.K2_AttachToActor` _returnvalue_2 self "None" "KeepWorld" "KeepWorld" "KeepWorld" true)
          (`self.Push`))))))

(event `Push`
  (bind _returnvalue (`GameplayStatics.GetPlayerController` 0))
  (`|ExecutionSequence`
    (:`then_0`
      (set `self.CurrentLocation` (`self.K2_GetActorLocation`))
      (bind (_direction _newtrack_0) (`Timeline|Timeline` :!via `PlayFromStart`)
        (:`Update`
          (`self.K2_SetActorRelativeLocation` (+ (`self.CurrentLocation`) (* _newtrack_0 (`self.PushableDirection`) (`self.TravelDistance`)))))
        (:`Finished`
          (if (or (`PlayerController.IsInputKeyDown` _returnvalue "D") (`PlayerController.IsInputKeyDown` _returnvalue "W") (`PlayerController.IsInputKeyDown` _returnvalue "S") (`PlayerController.IsInputKeyDown` _returnvalue "A"))
            (bind _canpush (`self.CanPush`))
            (if _canpush
              (`self.Push`)
              (else
                (`self.StopPushing`)))
            (else
              (`self.StopPushing`))))))
    (:`then_1`
      (`ActorComponent.Activate` (`self.PS_Sparks`) true)
      (`ActorComponent.Activate` (`self.PS_Sparks1`) true))))

(event `StopPushing`
  (bind _returnvalue (`GameplayStatics.GetPlayerCharacter` 0))
  (`|ExecutionSequence`
    (:`then_0`
      (`CharacterMovementComponent.SetMovementMode` (`Character.CharacterMovement` _returnvalue) "MOVE_Walking" 0)
      (`self.K2_DetachFromActor` _returnvalue "KeepWorld" "KeepWorld" "KeepWorld")
      (`CapsuleComponent.SetCapsuleRadius` (`Character.CapsuleComponent` _returnvalue) 35.0 true))
    (:`then_1`
      (`ActorComponent.Deactivate` (`self.PS_Sparks`))
      (`ActorComponent.Deactivate` (`self.PS_Sparks1`)))))

(fn `CanPush`
  (returns (CanPush :type Boolean))
  (locals (LocalCanPush :type Boolean :default true))
  (bind _returnvalue (`GameplayStatics.GetPlayerCharacter` 0))
  (bind _returnvalue_2 (`self.K2_GetActorLocation`))
  (bind _returnvalue_3 (`self.K2_GetActorLocation` _returnvalue))
  (bind (_returnvalue_origin _returnvalue_boxextent) (`KismetMathLibrary.BreakBoxSphereBounds` (`StaticMesh.GetBounds` (`StaticMeshComponent.StaticMesh` (`self.StaticMesh`)))))
  (bind _returnvalue_4 (+ (`self.K2_GetActorLocation`) (* (`self.PushableDirection`) (`self.TravelDistance`)) (0.0 0.0 0.0)))
  (`|ExecutionSequence`
    (:`then_0`
      ;[1 1 1 1 45] Check Player Facing Box
      (bind (_outhit _returnvalue_5) (`KismetSystemLibrary.LineTraceSingle` _returnvalue_3 (+ _returnvalue_3 (* (`self.GetActorForwardVector` _returnvalue) 100.0)) "TraceTypeQuery1" false (`|MakeArray` _returnvalue :!type "Actor Object Reference") "None" false))
      (if _returnvalue_5
        (if (not (== (`.HitActor` (`GameplayStatics.BreakHitResult` _outhit)) self))
          (set `local.LocalCanPush` false))
        (else
          (set `local.LocalCanPush` false))))
    (:`then_1`
      ;[1 1 1 1 50] Check if Box has Room to Move
      (bind (_outhit_2 _returnvalue_6) (`KismetSystemLibrary.BoxTraceSingle` (+ _returnvalue_2 (0.0 0.0 120.0)) (+ _returnvalue_2 (* (`self.PushableDirection`) (`self.TravelDistance`)) (0.0 0.0 120.0)) (* _returnvalue_boxextent 1.0) (struct) "TraceTypeQuery1" false (`|MakeArray` self :!type "Actor Object Reference")))
      (if (not (not _returnvalue_6))
        (set `local.LocalCanPush` false)))
    (:`then_2`
      ;[1 1 1 1 50] Check For Floor
      (bind (_outhit_3 _returnvalue_7) (`KismetSystemLibrary.LineTraceSingle` _returnvalue_4 (+ _returnvalue_4 (0.0 0.0 -150.0)) "TraceTypeQuery1"))
      (if (not _returnvalue_7)
        (set `local.LocalCanPush` false)))
    (:`then_3`
      ;[1 1 1 1 45] Check if Player Jumping
      (if (`NavMovementComponent.IsFalling` (`Character.CharacterMovement` (`GameplayStatics.GetPlayerCharacter` 0)))
        (set `local.LocalCanPush` false)))
    (:`then_4`
      (if (`/Game/Blueprints/Class/BP_Robot.GunEquipped` (`self.As BP Robot`))
        (set `local.LocalCanPush` false)))
    (:`then_5`
      (return (`local.LocalCanPush`)))))

(fn `UserConstructionScript`)