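; BP_Camera is a cine camera actor that switches between two fixed preset shots.
; Custom events Move1 and Move2 each snap instantly to a hard-coded world position, rotation and focal length, with no blending.
; Move1 relocates the scene root while Move2 relocates only the CineCamera component; both rotate the camera component.
; Nothing in the actor triggers these events, and BeginPlay, Tick and the construction script are empty.
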(event `Move1`
  (`SceneComponent.K2_SetWorldLocation` (`self.DefaultSceneRoot`) (-1490.68064 817.362273 471.313322) false false)
  (`SceneComponent.K2_SetWorldRotation` (`self.CineCamera`) (struct :`Pitch` 338.0) false false)
  (set `CineCameraComponent.CurrentFocalLength` 35.0 (`self.CineCamera`)))

(event `Move2`
  (`SceneComponent.K2_SetWorldLocation` (`self.CineCamera`) (463.662202 529.204549 810.08992) false false)
  (`SceneComponent.K2_SetWorldRotation` (`self.CineCamera`) (struct :`Pitch` -32.0 :`Yaw` 320.0) false false)
  (set `CineCameraComponent.CurrentFocalLength` 16.0 (`self.CineCamera`)))

(fn `UserConstructionScript`)