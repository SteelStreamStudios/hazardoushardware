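; BP_FenceDoor is a skeletal mesh fence door with a glowing, color-coded material that can be opened.
; On BeginPlay it creates a dynamic instance of each mesh material and stores them, then SetValues pushes the Glow and Color parameters to all of them.
; OpenDoor turns the color green, waits briefly, plays the opening animation and disables the mesh's collision.
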(event `self.ReceiveBeginPlay`
  (bind _sk_fencedoor (`self.SK_FenceDoor`))
  (for (_array_element _array_index) (`MeshComponent.GetMaterials` _sk_fencedoor)
    (bind _returnvalue (`PrimitiveComponent.CreateDynamicMaterialInstance` _sk_fencedoor _array_index _array_element "None"))
    (`KismetArrayLibrary.Array_Set` (`self.Target Array`) _array_index _returnvalue true))
  (`self.SetValues`))

(event `SetValues`
  (for _array_element (`self.Target Array`)
    (`MaterialInstanceDynamic.SetScalarParameterValue` _array_element "Glow" (`self.Glow`))
    (`MaterialInstanceDynamic.SetVectorParameterValue` _array_element "Color" (`self.Color`))))

(event `OpenDoor`
  (set `self.Color` (struct :`R` 0.087081 :`G` 1.0 :`A` 1.0))
  (`self.SetValues`)
  (`KismetSystemLibrary.Delay` 1.0)
  (`SkeletalMeshComponent.PlayAnimation` (`self.SK_FenceDoor`) "/Game/Meshes/Environment/A_FenceDoorOpen.A_FenceDoorOpen" false)
  (`PrimitiveComponent.SetCollisionEnabled` (`self.SK_FenceDoor`) "NoCollision"))

(fn `UserConstructionScript`)