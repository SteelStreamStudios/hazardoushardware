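; Destructible wall set piece that blows up once when a projectile hits its trigger box while the player robot is in the janitor closet.
; The blast enables wall physics, spawns a Niagara explosion and fires three staggered projectiles with hidden spheres from an arrow component.
; It then hides the barrels and pallets, disables their collision and, after a short delay, calls PushChair on the level's BP_Chair.
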(event `self.ReceiveBeginPlay`)

(event `self.Box.OnComponentBeginOverlap`
  (params (OverlappedComponent :type "PrimitiveComponent Object Reference") (OtherActor :type "Actor Object Reference") (OtherComp :type "PrimitiveComponent Object Reference") (OtherBodyIndex :type Integer) (bFromSweep :type Boolean) (SweepResult :type "HitResult Structure (by ref)"))
  (bind (_returnvalue_location _returnvalue_rotation) (`KismetMathLibrary.BreakTransform` (`SceneComponent.K2_GetComponentToWorld` (`self.Arrow`))))
  (bind (_returnvalue_location_2 _returnvalue_rotation_2) (`KismetMathLibrary.BreakTransform` (`SceneComponent.K2_GetComponentToWorld` (`self.Arrow`))))
  (bind (_returnvalue_location_3 _returnvalue_rotation_3) (`KismetMathLibrary.BreakTransform` (`SceneComponent.K2_GetComponentToWorld` (`self.Arrow`))))
  (cast `/Game/Blueprints/Class/BP_Projectile` OtherActor)
  (bind _asbp_robot (cast `/Game/Blueprints/Class/BP_Robot` (`GameplayStatics.GetPlayerPawn` 0)))
  (if (`/Game/Blueprints/Class/BP_Robot.InJanitorCloset` _asbp_robot)
    (`/Engine/EditorBlueprintResources/StandardMacros.DoOnce` false
      (:`Completed`
        (`PrimitiveComponent.SetSimulatePhysics` (`self.Wall`) true)
        (`NiagaraFunctionLibrary.SpawnSystemAtLocation` "/Game/VFX/PS_LargeExplosion1.PS_LargeExplosion1" (`SceneComponent.K2_GetComponentLocation` (`self.Pallet`)))
        (bind _returnvalue (`|SpawnActorFromClass` "/Game/Blueprints/Class/BP_Projectile.BP_Projectile_C" (`KismetMathLibrary.MakeTransform` _returnvalue_location _returnvalue_rotation) "Undefined" "MultiplyWithRoot" null null))
        (`SceneComponent.SetVisibility` (`/Game/Blueprints/Class/BP_Projectile.Sphere` _returnvalue) false false)
        (`KismetSystemLibrary.Delay` 0.2)
        (bind _returnvalue_2 (`|SpawnActorFromClass` "/Game/Blueprints/Class/BP_Projectile.BP_Projectile_C" (`KismetMathLibrary.MakeTransform` _returnvalue_location_2 _returnvalue_rotation_2) "Undefined" "MultiplyWithRoot" null null))
        (`SceneComponent.SetVisibility` (`/Game/Blueprints/Class/BP_Projectile.Sphere` _returnvalue_2) false false)
        (`KismetSystemLibrary.Delay` 0.2)
        (bind _returnvalue_3 (`|SpawnActorFromClass` "/Game/Blueprints/Class/BP_Projectile.BP_Projectile_C" (`KismetMathLibrary.MakeTransform` _returnvalue_location_3 _returnvalue_rotation_3) "Undefined" "MultiplyWithRoot" null null))
        (`SceneComponent.SetVisibility` (`/Game/Blueprints/Class/BP_Projectile.Sphere` _returnvalue_3) false false)
        (`SceneComponent.SetVisibility` (`self.Pallet`) false false)
        (`SceneComponent.SetVisibility` (`self.Barrel3`) false false)
        (`SceneComponent.SetVisibility` (`self.Barrel1`) false false)
        (`SceneComponent.SetVisibility` (`self.Barrel`) false false)
        (`SceneComponent.SetVisibility` (`self.Barrel2`) false false)
        (`SceneComponent.SetVisibility` (`self.Pallet1`) false false)
        (`SceneComponent.SetVisibility` (`self.Barrel7`) false false)
        (`SceneComponent.SetVisibility` (`self.Barrel5`) false false)
        (`SceneComponent.SetVisibility` (`self.Barrel6`) false false)
        (`SceneComponent.SetVisibility` (`self.Barrel4`) false false)
        (`PrimitiveComponent.SetCollisionEnabled` (`self.Barrel4`) "NoCollision")
        (`PrimitiveComponent.SetCollisionEnabled` (`self.Barrel6`) "NoCollision")
        (`PrimitiveComponent.SetCollisionEnabled` (`self.Barrel5`) "NoCollision")
        (`PrimitiveComponent.SetCollisionEnabled` (`self.Barrel7`) "NoCollision")
        (`PrimitiveComponent.SetCollisionEnabled` (`self.Pallet1`) "NoCollision")
        (`PrimitiveComponent.SetCollisionEnabled` (`self.Barrel2`) "NoCollision")
        (`PrimitiveComponent.SetCollisionEnabled` (`self.Barrel`) "NoCollision")
        (`PrimitiveComponent.SetCollisionEnabled` (`self.Barrel1`) "NoCollision")
        (`PrimitiveComponent.SetCollisionEnabled` (`self.Barrel3`) "NoCollision")
        (`PrimitiveComponent.SetCollisionEnabled` (`self.Pallet`) "NoCollision")
        (`KismetSystemLibrary.Delay` 0.25)
        (bind _returnvalue_4 (`GameplayStatics.GetActorOfClass` "/Game/Blueprints/Class/BP_Chair.BP_Chair_C"))
        (`/Game/Blueprints/Class/BP_Chair.PushChair` _returnvalue_4)))))

(fn `UserConstructionScript`)