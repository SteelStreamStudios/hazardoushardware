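; BP_Divider is an actor with two indicator lights that show red or green status for an explosive barrel.
; BeginPlay creates dynamic material instances for both lights and starts them dark.
; PowerOn and BarrelDestroyed light the first one red and turn the second off.
; A BP_ExplosiveBarrel entering the Box trigger turns off the red light and lights the second one green.
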(event `self.ReceiveBeginPlay`
  (bind _light1 (`self.Light1`))
  (bind _light2 (`self.Light2`))
  (bind _returnvalue (`PrimitiveComponent.CreateDynamicMaterialInstance` _light1 0 (`PrimitiveComponent.GetMaterial` _light1 0) "None"))
  (bind _output_get (set `self.Light1Mat` _returnvalue))
  (`MaterialInstanceDynamic.SetScalarParameterValue` _output_get "Glow" 0.0)
  (`MaterialInstanceDynamic.SetVectorParameterValue` :`self` _output_get :`ParameterName` "Color")
  (bind _returnvalue_2 (`PrimitiveComponent.CreateDynamicMaterialInstance` _light2 0 (`PrimitiveComponent.GetMaterial` _light2 0) "None"))
  (bind _output_get_2 (set `self.Light2Mat` _returnvalue_2))
  (`MaterialInstanceDynamic.SetScalarParameterValue` _output_get_2 "Glow" 0.0)
  (`MaterialInstanceDynamic.SetVectorParameterValue` :`self` _output_get_2 :`ParameterName` "Color"))

(event `self.Box.OnComponentBeginOverlap`
  (params (OverlappedComponent :type "PrimitiveComponent Object Reference") (OtherActor :type "Actor Object Reference") (OtherComp :type "PrimitiveComponent Object Reference") (OtherBodyIndex :type Integer) (bFromSweep :type Boolean) (SweepResult :type "HitResult Structure (by ref)"))
  (bind _light2mat (`self.Light2Mat`))
  (cast `/Game/Blueprints/Class/BP_ExplosiveBarrel` OtherActor)
  (`MaterialInstanceDynamic.SetScalarParameterValue` (`self.Light1Mat`) "Glow" 0.0)
  (`MaterialInstanceDynamic.SetScalarParameterValue` _light2mat "Glow" 5.0)
  (`MaterialInstanceDynamic.SetVectorParameterValue` _light2mat "Color" (struct :`G` 1.0 :`B` 0.019322 :`A` 1.0)))

(event `PowerOn`
  (bind _light1mat (`self.Light1Mat`))
  (bind _light2mat (`self.Light2Mat`))
  (`MaterialInstanceDynamic.SetScalarParameterValue` _light1mat "Glow" 5.0)
  (`MaterialInstanceDynamic.SetVectorParameterValue` _light1mat "Color" (struct :`R` 1.0 :`G` 0.011936 :`A` 1.0))
  (`MaterialInstanceDynamic.SetScalarParameterValue` _light2mat "Glow" 0.0)
  (`MaterialInstanceDynamic.SetVectorParameterValue` _light2mat "Color" (struct :`A` 1.0)))

(event `BarrelDestroyed`
  (bind _light1mat (`self.Light1Mat`))
  (bind _light2mat (`self.Light2Mat`))
  (`MaterialInstanceDynamic.SetScalarParameterValue` _light1mat "Glow" 5.0)
  (`MaterialInstanceDynamic.SetVectorParameterValue` _light1mat "Color" (struct :`R` 1.0 :`G` 0.011936 :`A` 1.0))
  (`MaterialInstanceDynamic.SetScalarParameterValue` _light2mat "Glow" 0.0)
  (`MaterialInstanceDynamic.SetVectorParameterValue` _light2mat "Color" (struct :`A` 1.0)))

(fn `UserConstructionScript`)