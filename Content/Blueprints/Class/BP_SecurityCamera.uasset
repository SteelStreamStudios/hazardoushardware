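; Security camera that sweeps back and forth and triggers a facility-wide lockdown when the player enters its detection sphere.
; Two timelines alternate the yaw scan until detection calls LockdownStart on every camera, halting scans, reddening spotlights, locking doors, and alerting laser bots and the console.
; Cameras with First set also play a view-blend cutscene with input disabled.
; LockdownEnd restores scanning and re-arms detection through paired DoOnce gates.
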(event `self.ReceiveBeginPlay`
  (`KismetSystemLibrary.Delay` (`self.Delay`))
  (`self.CameraScan`))

(event `CameraScan`
  (bind _camera (`self.Camera`))
  (bind _camera_2 (`self.Camera`))
  (bind (_returnvalue_roll _returnvalue_pitch _returnvalue_yaw) (`KismetMathLibrary.BreakRotator` (`SceneComponent.K2_GetComponentRotation` _camera)))
  (bind (_returnvalue_roll_2 _returnvalue_pitch_2 _returnvalue_yaw_2) (`KismetMathLibrary.BreakRotator` (`SceneComponent.K2_GetComponentRotation` _camera_2)))
  (if (`self.Spotted`)
    _
    (elif (`self.Reverse`)
      (if (`self.Finished`)
        (bind (_direction _newtrack_0) (`Timeline|Timeline_0` :!via `PlayFromStart` :!label _label)
          (:`Update`
            (set `self.Finished` false)
            (`SceneComponent.K2_SetWorldRotation` _camera (`KismetMathLibrary.MakeRotator` _returnvalue_roll _returnvalue_pitch (+ _returnvalue_yaw _newtrack_0)) false false))
          (:`Finished`
            (set `self.Reverse` false)
            (set `self.Finished` true)
            (`KismetSystemLibrary.RetriggerableDelay` 0.2)
            (`self.CameraScan`)))
        (else
          (goto _label)))
      (elif (`self.Finished`)
        (bind (_direction_2 _newtrack_0_2) (`Timeline|Timeline` :!via `PlayFromStart` :!label _label_2)
          (:`Update`
            (set `self.Finished` false)
            (`SceneComponent.K2_SetWorldRotation` _camera_2 (`KismetMathLibrary.MakeRotator` _returnvalue_roll_2 _returnvalue_pitch_2 (+ _returnvalue_yaw_2 _newtrack_0_2)) false false))
          (:`Finished`
            (set `self.Reverse` true)
            (set `self.Finished` true)
            (`KismetSystemLibrary.RetriggerableDelay` 0.2)
            (`self.CameraScan`)))
        (else
          (goto _label_2))))))

(event `LockdownStart`
  (bind _returnvalue (`GameplayStatics.GetPlayerController` 0))
  (bind _returnvalue_2 (`GameplayStatics.GetPlayerController` 0))
  (bind _returnvalue_3 (`GameplayStatics.GetPlayerPawn` 0))
  (`LightComponent.SetLightColor` (`self.SpotLight`) (struct :`R` 1.0 :`B` 0.006452 :`A` 1.0) true)
  (set `self.Spotted` true)
  (if (`self.First`)
    (`self.DisableInput` (`GameplayStatics.GetPlayerPawn` 0) _returnvalue)
    (bind _returnvalue_4 (`GameplayStatics.GetActorOfClass` "/Game/Blueprints/Class/BP_Camera2.BP_Camera2_C"))
    (`PlayerController.SetViewTargetWithBlend` _returnvalue _returnvalue_4 3.0 "VTBlend_EaseInOut" 2.0 false)
    (`KismetSystemLibrary.Delay` 3.0)
    (bind _outactors (`GameplayStatics.GetAllActorsOfClass` "/Game/Blueprints/Class/BP_SecurityDoor.BP_SecurityDoor_C"))
    (for _array_element _outactors
      (`/Game/Blueprints/Class/BP_SecurityDoor.LockDoor` _array_element))
    (`KismetSystemLibrary.Delay` 2.2)
    (`PlayerController.SetViewTargetWithBlend` _returnvalue_2 _returnvalue_3 3.0 "VTBlend_EaseInOut" 2.0 false)
    (`KismetSystemLibrary.Delay` 3.0)
    (`self.EnableInput` _returnvalue_3 _returnvalue_2))
  (`|ExecutionSequence`
    (:`then_0`
      (goto _label :!via `Stop`))
    (:`then_1`
      (goto _label_2 :!via `Stop`))
    (:`then_2`
      (goto _label_4 :!via `Reset`))
    (:`then_3`
      (bind _outactors_2 (`GameplayStatics.GetAllActorsOfClass` "/Game/Blueprints/Class/BP_LaserBot.BP_LaserBot_C"))
      (for _array_element_2 _outactors_2
        (`/Game/Blueprints/Class/BP_LaserBot.Attack` _array_element_2)
        (set `/Game/Blueprints/Class/BP_LaserBot.Lockdown` true _array_element_2)))
    (:`then_4`
      (if (`self.First`)
        (set `self.First` false)
        (else
          (bind _outactors_3 (`GameplayStatics.GetAllActorsOfClass` "/Game/Blueprints/Class/BP_SecurityDoor.BP_SecurityDoor_C"))
          (for _array_element_3 _outactors_3
            (`/Game/Blueprints/Class/BP_SecurityDoor.LockDoor` _array_element_3)))))
    (:`then_5`
      (bind _returnvalue_5 (`GameplayStatics.GetActorOfClass` "/Game/Blueprints/Class/BP_SecurityConsole.BP_SecurityConsole_C"))
      (`/Game/Blueprints/Class/BP_SecurityConsole.LockDown` _returnvalue_5))))

(event `self.Sphere.OnComponentBeginOverlap`
  (params (OverlappedComponent :type "PrimitiveComponent Object Reference") (OtherActor :type "Actor Object Reference") (OtherComp :type "PrimitiveComponent Object Reference") (OtherBodyIndex :type Integer) (bFromSweep :type Boolean) (SweepResult :type "HitResult Structure (by ref)"))
  (if (== OtherActor (`GameplayStatics.GetPlayerPawn` 0))
    (`/Engine/EditorBlueprintResources/StandardMacros.DoOnce` false :!label _label_3
      (:`Completed`
        (bind _outactors (`GameplayStatics.GetAllActorsOfClass` "BP_SecurityCamera_C"))
        (for _array_element _outactors
          (`self.LockdownStart` _array_element))))))

(event `LockdownEnd`
  (`/Engine/EditorBlueprintResources/StandardMacros.DoOnce` false :!label _label_4
    (:`Completed`
      (`LightComponent.SetLightColor` (`self.SpotLight`) (struct :`R` 1.0 :`G` 1.0 :`B` 1.0 :`A` 1.0) true)
      (set `self.Spotted` false)
      (`self.CameraScan`)
      (goto _label_3 :!via `Reset`))))

(fn `UserConstructionScript`)