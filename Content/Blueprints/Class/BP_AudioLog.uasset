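; BP_AudioLog is a collectible audio log with an animated "Press E" prompt for the player.
; Sphere overlap scales the prompt Plane in and out through two timelines, gated by paired DoOnce nodes.
; PickUp uses AudioLogNum to select one of four logs, plays it as 2D sound with a camera shutter, flags it collected in BP_GameState, then destroys the actor.
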(event `self.ReceiveBeginPlay`
  (bind _asbp_game_state (cast `/Game/Blueprints/Class/BP_GameState` (`GameplayStatics.GetGameState`)))
  (set `self.GameState` _asbp_game_state))

(event `self.Sphere.OnComponentBeginOverlap`
  (params (OverlappedComponent :type "PrimitiveComponent Object Reference") (OtherActor :type "Actor Object Reference") (OtherComp :type "PrimitiveComponent Object Reference") (OtherBodyIndex :type Integer) (bFromSweep :type Boolean) (SweepResult :type "HitResult Structure (by ref)"))
  ;[1 1 1] "Press E" Prompt Active
  (if (== OtherActor (`GameplayStatics.GetPlayerPawn` 0))
    (`/Engine/EditorBlueprintResources/StandardMacros.DoOnce` false :!label _label
      (:`Completed`
        (`|ExecutionSequence`
          (:`then_0`
            ;[1 1 1] "Press E" Prompt Deactive
            (bind (_direction _time) (`Timeline|Timeline_0` :!via `Stop` :!label _label_2)
              (:`Update`
                (`SceneComponent.SetWorldScale3D` (`self.Plane`) (`KismetMathLibrary.VLerp` (2.8 2.8 2.8) (0.0 0.0 0.0) _time)))))
          (:`then_1`
            (bind (_direction_2 _time_2) (`Timeline|Timeline` :!via `PlayFromStart` :!label _label_3)
              (:`Update`
                (`SceneComponent.SetWorldScale3D` (`self.Plane`) (`KismetMathLibrary.VLerp` (0.0 0.0 0.0) (2.8 2.8 2.8) _time_2)))))
          (:`then_2`
            (goto _label_4 :!via `Reset`)))))))

(event `self.Sphere.OnComponentEndOverlap`
  (params (OverlappedComponent :type "PrimitiveComponent Object Reference") (OtherActor :type "Actor Object Reference") (OtherComp :type "PrimitiveComponent Object Reference") (OtherBodyIndex :type Integer))
  ;[1 1 1] "Press E" Prompt Deactive
  (if (== OtherActor (`GameplayStatics.GetPlayerPawn` 0))
    (`/Engine/EditorBlueprintResources/StandardMacros.DoOnce` true :!label _label_4
      (:`Completed`
        (`|ExecutionSequence`
          (:`then_0`
            (goto _label_3 :!via `Stop`))
          (:`then_1`
            (goto _label_2 :!via `PlayFromStart`))
          (:`then_2`
            (goto _label :!via `Reset`)))))))

(event `/Game/Blueprints/Interfaces/BP_PickUpInterface.PickUp`
  (if (== (`self.AudioLogNum`) 1)
    (`GameplayStatics.PlaySound2D` "/Engine/VREditor/Sounds/UI/Camera_Shutter.Camera_Shutter" 1.0 1.0 0.0 null null)
    (`GameplayStatics.PlaySound2D` "/Game/Audio/Dialoge/AudioLog1.AudioLog1" 1.0 1.0 0.0 null null)
    (set `/Game/Blueprints/Class/BP_GameState.AudioLog1PickedUp` true (`self.GameState`))
    (`self.K2_DestroyActor`)
    (elif (== (`self.AudioLogNum`) 2)
      (`GameplayStatics.PlaySound2D` "/Engine/VREditor/Sounds/UI/Camera_Shutter.Camera_Shutter" 1.0 1.0 0.0 null null)
      (`GameplayStatics.PlaySound2D` "/Game/Audio/Dialoge/AudioLog2.AudioLog2" 1.0 1.0 0.0 null null)
      (set `/Game/Blueprints/Class/BP_GameState.AudioLog2PickedUp` true (`self.GameState`))
      (`self.K2_DestroyActor`)
      (elif (== (`self.AudioLogNum`) 3)
        (`GameplayStatics.PlaySound2D` "/Engine/VREditor/Sounds/UI/Camera_Shutter.Camera_Shutter" 1.0 1.0 0.0 null null)
        (`GameplayStatics.PlaySound2D` "/Game/Audio/Dialoge/AudioLog3.AudioLog3" 1.0 1.0 0.0 null null)
        (set `/Game/Blueprints/Class/BP_GameState.AudioLog3PickedUp` true (`self.GameState`))
        (`self.K2_DestroyActor`)
        (elif (== (`self.AudioLogNum`) 4)
          (`GameplayStatics.PlaySound2D` "/Engine/VREditor/Sounds/UI/Camera_Shutter.Camera_Shutter" 1.0 1.0 0.0 null null)
          (`GameplayStatics.PlaySound2D` "/Game/Audio/Dialoge/AudioLog4.AudioLog4" 1.0 1.0 0.0 null null)
          (set `/Game/Blueprints/Class/BP_GameState.AudioLog4PickedUp` true (`self.GameState`))
          (`self.K2_DestroyActor`))))))

(fn `UserConstructionScript`)