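; Missile turret that spots the player's BP_Robot with PawnSensing, yaws to track it and calls MissileStrike on it after a delay.
; Dynamic materials show alert state by color and power state by glow, while timelines drive a Time value for the aim animation blend.
; DoOnce gates space out attacks, the alert clears if the robot is behind cover afterward, and PowerDown/PowerUp events toggle sensing and glow.
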(event `self.ReceiveBeginPlay`
  (bind _base (`self.Base`))
  (bind _asbp_robot (cast `/Game/Blueprints/Class/BP_Robot` (`GameplayStatics.GetPlayerPawn` 0)))
  (set `self.As Robot BP` _asbp_robot)
  ;[1 1 1] Colour Change
  (for (_array_element _array_index) (`MeshComponent.GetMaterials` _base)
    (bind _returnvalue (`PrimitiveComponent.CreateDynamicMaterialInstance` _base _array_index _array_element "None"))
    (`KismetArrayLibrary.Array_Set` (`self.MatArray`) _array_index _returnvalue true))
  (`self.SetValues`))

(event `SetValues`
  ;[1 1 1] Colour Change
  (for _array_element (`self.MatArray`)
    (`MaterialInstanceDynamic.SetScalarParameterValue` _array_element "Glow" (`self.Glow`))
    (`MaterialInstanceDynamic.SetVectorParameterValue` _array_element "Color" (`self.Color`))))

(event `self.PawnSensing.OnSeePawn`
  (params (Pawn :type "Pawn Object Reference"))
  ;[1 1 1] Pawn Sensing
  (if (== Pawn (`GameplayStatics.GetPlayerPawn` 0))
    (`|ExecutionSequence`
      (:`then_0`
        (set `self.Color` (struct :`R` 1.0 :`G` 0.032358 :`A` 1.0))
        (set `self.Spotted` true)
        (`self.SetValues`)
        (if (not (`self.Aiming`))
          (`self.TimeIncrease`)
          (set `self.Aiming` true)))
      (:`then_1`
        (`/Engine/EditorBlueprintResources/StandardMacros.DoOnce` false :!label _label
          (:`Completed`
            (`KismetSystemLibrary.Delay` 1.0)
            (`self.Fire`)
            (`KismetSystemLibrary.Delay` 4.0)
            (if (`/Game/Blueprints/Class/BP_Robot.IsBehindCover?` (`self.As Robot BP`))
              (set `self.Spotted` false)
              (set `self.Color` (struct :`G` 1.0 :`B` 0.004274 :`A` 1.0))
              (`self.SetValues`)
              (goto _label :!via `Reset`)
              (else
                (goto _label :!via `Reset`)))))))))

(event `TimeIncrease`
  ;[1 1 1] Anim Blend
  (bind (_direction _newtrack_0) (`Timeline|Timeline` :!via `PlayFromStart`)
    (:`Update`
      (set `self.Time` _newtrack_0))))

(event `Fire`
  ;[1 1 1] Fire
  (`/Engine/EditorBlueprintResources/StandardMacros.DoOnce` false :!label _label_2
    (:`Completed`
      (set `self.Firing` true)
      (`KismetSystemLibrary.Delay` 2.0)
      (set `self.Firing` false)
      (`|ExecutionSequence`
        (:`then_0`
          (`/Game/Blueprints/Class/BP_Robot.MissileStrike` (`self.As Robot BP`)))
        (:`then_1`
          (goto _label_2 :!via `Reset`))))))

(event `self.ReceiveTick`
  (params (DeltaSeconds :type "Float (single-precision)"))
  (bind (_returnvalue_roll _returnvalue_pitch _returnvalue_yaw) (`KismetMathLibrary.BreakRotator` (`KismetMathLibrary.FindLookAtRotation` (`SceneComponent.K2_GetComponentLocation` (`self.Turret`)) (`SceneComponent.K2_GetComponentLocation` (`Character.Mesh` (`self.As Robot BP`))))))
  ;[1 1 1] Event Tick
  (if (`self.Spotted`)
    (`SceneComponent.K2_SetWorldRotation` (`self.Turret`) (`KismetMathLibrary.MakeRotator` 0.0 0.0 (+ _returnvalue_yaw -90.0)) false false)))

(event `PowerDown`
  (`/Engine/EditorBlueprintResources/StandardMacros.DoOnce` false :!label _label_3
    (:`Completed`
      (set `PawnSensingComponent.bSeePawns` false (`self.PawnSensing`))
      (set `self.Glow` 0.0)
      (`self.SetValues`)
      (set `self.Time` 0.0)
      (bind (_direction _newtrack_0) (`Timeline|Timeline_0` :!via `PlayFromStart`)
        (:`Update`
          (set `self.Time` _newtrack_0)
          (goto _label_4 :!via `Reset`))))))

(event `PowerUp`
  (`/Engine/EditorBlueprintResources/StandardMacros.DoOnce` false :!label _label_4
    (:`Completed`
      (set `PawnSensingComponent.bSeePawns` true (`self.PawnSensing`))
      (set `self.Glow` 10.0)
      (`self.SetValues`)
      (set `self.Time` 100.0)
      (bind (_direction _newtrack_0) (`Timeline|Timeline_1` :!via `PlayFromStart`)
        (:`Update`
          (set `self.Time` _newtrack_0)
          (goto _label_3 :!via `Reset`))))))

(fn `UserConstructionScript`)