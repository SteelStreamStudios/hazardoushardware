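; BP_ElectricFloorSound is a Blueprint that provides repeating audio, by its name for an electric floor.
; From BeginPlay, the Sound event plays Electricity through Buzz, waits a fixed delay, then plays SwitchSound through Switch.
; Sound then calls itself, so the buzz and switch cycle repeats endlessly with no Tick or stop condition.
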(event `Sound`
  (`self.Buzz`)
  (`KismetSystemLibrary.Delay` 4.5)
  (`self.Switch`)
  (`self.Sound`))

(event `self.ReceiveBeginPlay`
  (`self.Sound`))

(event `Switch`
  (`AudioComponent.Play` (`self.SwitchSound`) 0.0))

(event `Buzz`
  (`AudioComponent.Play` (`self.Electricity`) 0.0))

(fn `UserConstructionScript`)