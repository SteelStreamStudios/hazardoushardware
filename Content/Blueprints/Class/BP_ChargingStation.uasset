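; Charging station that heals the player's BP_Robot and serves as a respawn checkpoint.
; Player overlap turns its dynamic material green, plays power-up effects, heals the robot and makes this active station the sole checkpoint among all stations.
; Paired DoOnce gates limit this to once per visit, with overlap end turning it red and inactive.
; RespawnPlayer plays respawn effects and a brief blue glow on the checkpoint station.
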(event `self.ReceiveBeginPlay`
  (bind _chargingstation (`self.ChargingStation`))
  (bind _returnvalue (`PrimitiveComponent.CreateDynamicMaterialInstance` _chargingstation 0 (`PrimitiveComponent.GetMaterial` _chargingstation 0) "None"))
  (set `self.Material` _returnvalue))

(event `self.Capsule.OnComponentBeginOverlap`
  (params (OverlappedComponent :type "PrimitiveComponent Object Reference") (OtherActor :type "Actor Object Reference") (OtherComp :type "PrimitiveComponent Object Reference") (OtherBodyIndex :type Integer) (bFromSweep :type Boolean) (SweepResult :type "HitResult Structure (by ref)"))
  (bind _returnvalue (`GameplayStatics.GetPlayerPawn` 0))
  (if (== OtherActor _returnvalue)
    (`MaterialInstanceDynamic.SetVectorParameterValue` (`self.Material`) "Emissive_Color" (struct :`G` 1.0 :`B` 0.011662 :`A` 1.0))
    (`/Engine/EditorBlueprintResources/StandardMacros.DoOnce` false :!label _label
      (:`Completed`
        (set `self.IsActive` true)
        (bind _asbp_robot (cast `/Game/Blueprints/Class/BP_Robot` _returnvalue))
        (`GameplayStatics.PlaySound2D` "/Game/Audio/Level2/Charging_station_Power_up.Charging_station_Power_up" 0.4 1.0 0.0 null null)
        (if (< (`/Game/Blueprints/Class/BP_Robot.CurrentHealth` _asbp_robot) 3.0)
          (`ActorComponent.Activate` (`self.Charging`) true)
          (`/Game/Blueprints/Class/BP_Robot.Heal` _asbp_robot)
          (else
            (`ActorComponent.Activate` (`self.Charging`) true)
            (`/Game/Blueprints/UI/BP_Health_Widget.FullHealth` (`/Game/Blueprints/Class/BP_Robot.Health` _asbp_robot))))
        (bind _outactors (`GameplayStatics.GetAllActorsOfClass` "BP_ChargingStation_C"))
        (for _array_element _outactors
          (if (`/Game/Blueprints/Class/BP_ChargingStation.IsActive` _array_element)
            (set `/Game/Blueprints/Class/BP_ChargingStation.Checkpoint` true _array_element)
            (else
              (set `/Game/Blueprints/Class/BP_ChargingStation.Checkpoint` false _array_element))))
        (goto _label_2 :!via `Reset`)))))

(event `self.Capsule.OnComponentEndOverlap`
  (params (OverlappedComponent :type "PrimitiveComponent Object Reference") (OtherActor :type "Actor Object Reference") (OtherComp :type "PrimitiveComponent Object Reference") (OtherBodyIndex :type Integer))
  (if (== OtherActor (`GameplayStatics.GetPlayerPawn` 0))
    (`/Engine/EditorBlueprintResources/StandardMacros.DoOnce` false :!label _label_2
      (:`Completed`
        (`MaterialInstanceDynamic.SetVectorParameterValue` (`self.Material`) "Emissive_Color" (struct :`R` 1.0 :`B` 0.008232 :`A` 1.0))
        (set `self.IsActive` false)
        (`ActorComponent.Deactivate` (`self.Charging`))
        (goto _label :!via `Reset`)))))

(event `RespawnPlayer`
  (if (`self.Checkpoint`)
    (`ActorComponent.Activate` (`self.Respawn`) true)
    (`MaterialInstanceDynamic.SetVectorParameterValue` (`self.Material`) "Emissive_Color" (struct :`G` 0.536032 :`B` 1.0 :`A` 1.0))
    (`GameplayStatics.PlaySound2D` "/Game/Audio/Level2/RespawnSound.RespawnSound" 1.0 1.0 0.0 null null)
    (`KismetSystemLibrary.Delay` 1.5)
    (if (`self.Checkpoint`)
      (`MaterialInstanceDynamic.SetVectorParameterValue` (`self.Material`) "Emissive_Color" (struct :`G` 1.0 :`B` 0.011662 :`A` 1.0))
      (else
        (`MaterialInstanceDynamic.SetVectorParameterValue` (`self.Material`) "Emissive_Color" (struct :`R` 1.0 :`B` 0.008232 :`A` 1.0))))))

(fn `UserConstructionScript`)