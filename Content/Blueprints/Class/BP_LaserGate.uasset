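; Laser gate hazard that disassembles any BP_Robot overlapping its Box trigger unless the robot's full shield is up.
; The construction script stretches four particle beams between marker components.
; While the player pawn is inside Box1, Tick line-traces three beams, clipping each at its impact point and raising spawn probability on hits.
; The top beam is never traced, and the traces are purely visual.
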(event `self.Box.OnComponentBeginOverlap`
  (params (OverlappedComponent :type "PrimitiveComponent Object Reference") (OtherActor :type "Actor Object Reference") (OtherComp :type "PrimitiveComponent Object Reference") (OtherBodyIndex :type Integer) (bFromSweep :type Boolean) (SweepResult :type "HitResult Structure (by ref)"))
  (bind _asbp_robot (cast `/Game/Blueprints/Class/BP_Robot` OtherActor))
  (if (not (`/Game/Blueprints/Class/BP_Robot.FullShieldUP` _asbp_robot))
    (`/Game/Blueprints/Class/BP_Robot.Disassemble` _asbp_robot)))

(event `self.Box1.OnComponentBeginOverlap`
  (params (OverlappedComponent :type "PrimitiveComponent Object Reference") (OtherActor :type "Actor Object Reference") (OtherComp :type "PrimitiveComponent Object Reference") (OtherBodyIndex :type Integer) (bFromSweep :type Boolean) (SweepResult :type "HitResult Structure (by ref)"))
  (if (== OtherActor (`GameplayStatics.GetPlayerPawn` 0))
    (set `self.NearGate` true)))

(event `self.Box1.OnComponentEndOverlap`
  (params (OverlappedComponent :type "PrimitiveComponent Object Reference") (OtherActor :type "Actor Object Reference") (OtherComp :type "PrimitiveComponent Object Reference") (OtherBodyIndex :type Integer))
  (if (== OtherActor (`GameplayStatics.GetPlayerPawn` 0))
    (set `self.NearGate` false)))

(event `self.ReceiveTick`
  (params (DeltaSeconds :type "Float (single-precision)"))
  (bind _laser2 (`self.Laser2`))
  (bind _laser2_2 (`self.Laser2`))
  (bind _laser3 (`self.Laser3`))
  (bind _laser (`self.Laser`))
  (bind _laser_2 (`self.Laser`))
  (if (`self.NearGate`)
    (`|ExecutionSequence`
      (:`then_0`
        (bind (_outhit _returnvalue) (`KismetSystemLibrary.LineTraceSingle` (`SceneComponent.K2_GetComponentLocation` (`self.LowerBeamStart`)) (`SceneComponent.K2_GetComponentLocation` (`self.LowerBeamEnd`)) "TraceTypeQuery4"))
        (if _returnvalue
          (`FXSystemComponent.SetVectorParameter` _laser2 "BeamEnd" (`.ImpactPoint` (`GameplayStatics.BreakHitResult` _outhit)))
          (`FXSystemComponent.SetFloatParameter` _laser2 "BeamSpawnProb" 90.0)
          (else
            (`FXSystemComponent.SetVectorParameter` _laser2_2 "BeamEnd" (`SceneComponent.K2_GetComponentLocation` (`self.LowerBeamEnd`)))
            (`FXSystemComponent.SetFloatParameter` _laser2_2 "BeamSpawnProb" 0.0))))
      (:`then_1`
        (bind (_outhit_2 _returnvalue_2) (`KismetSystemLibrary.LineTraceSingle` (`SceneComponent.K2_GetComponentLocation` (`self.BottomBeamStart`)) (`SceneComponent.K2_GetComponentLocation` (`self.BottomBeamEnd`)) "TraceTypeQuery4"))
        (if _returnvalue_2
          (`FXSystemComponent.SetVectorParameter` _laser3 "BeamEnd" (`.ImpactPoint` (`GameplayStatics.BreakHitResult` _outhit_2)))
          (`FXSystemComponent.SetFloatParameter` _laser3 "BeamSpawnProb" 90.0)
          (else
            (`FXSystemComponent.SetVectorParameter` _laser3 "BeamEnd" (`SceneComponent.K2_GetComponentLocation` (`self.BottomBeamEnd`)))
            (`FXSystemComponent.SetFloatParameter` _laser3 "BeamSpawnProb" 0.0))))
      (:`then_2`
        (bind (_outhit_3 _returnvalue_3) (`KismetSystemLibrary.LineTraceSingle` (`SceneComponent.K2_GetComponentLocation` (`self.UpperBeamStart`)) (`SceneComponent.K2_GetComponentLocation` (`self.UpperBeamEnd`)) "TraceTypeQuery4"))
        (if _returnvalue_3
          (`FXSystemComponent.SetVectorParameter` _laser_2 "BeamEnd" (`.ImpactPoint` (`GameplayStatics.BreakHitResult` _outhit_3)))
          (`FXSystemComponent.SetFloatParameter` _laser "BeamSpawnProb" 90.0)
          (else
            (`FXSystemComponent.SetVectorParameter` _laser_2 "BeamEnd" (`SceneComponent.K2_GetComponentLocation` (`self.UpperBeamEnd`)))
            (`FXSystemComponent.SetFloatParameter` _laser "BeamSpawnProb" 0.0)))))))

(fn `UserConstructionScript`
  (bind _laser1 (`self.Laser1`))
  (bind _laser3 (`self.Laser3`))
  (bind _laser2 (`self.Laser2`))
  (bind _laser (`self.Laser`))
  (`FXSystemComponent.SetVectorParameter` (`self.Laser`) "BeamStart" (`SceneComponent.K2_GetComponentLocation` (`self.UpperBeamStart`)))
  (`FXSystemComponent.SetVectorParameter` _laser "BeamEnd" (`SceneComponent.K2_GetComponentLocation` (`self.UpperBeamEnd`)))
  (`FXSystemComponent.SetFloatParameter` _laser "BeamSpawnProb" 0.0)
  (`FXSystemComponent.SetVectorParameter` _laser1 "BeamStart" (`SceneComponent.K2_GetComponentLocation` (`self.TopBeamStart`)))
  (`FXSystemComponent.SetFloatParameter` _laser1 "BeamSpawnProb" 0.0)
  (`FXSystemComponent.SetVectorParameter` (`self.Laser1`) "BeamEnd" (`SceneComponent.K2_GetComponentLocation` (`self.TopBeamEnd`)))
  (`FXSystemComponent.SetVectorParameter` (`self.Laser2`) "BeamStart" (`SceneComponent.K2_GetComponentLocation` (`self.LowerBeamStart`)))
  (`FXSystemComponent.SetVectorParameter` _laser2 "BeamEnd" (`SceneComponent.K2_GetComponentLocation` (`self.LowerBeamEnd`)))
  (`FXSystemComponent.SetFloatParameter` _laser2 "BeamSpawnProb" 0.0)
  (`FXSystemComponent.SetVectorParameter` (`self.Laser3`) "BeamStart" (`SceneComponent.K2_GetComponentLocation` (`self.BottomBeamStart`)))
  (`FXSystemComponent.SetVectorParameter` _laser3 "BeamEnd" (`SceneComponent.K2_GetComponentLocation` (`self.BottomBeamEnd`)))
  (`FXSystemComponent.SetFloatParameter` _laser3 "BeamSpawnProb" 0.0))