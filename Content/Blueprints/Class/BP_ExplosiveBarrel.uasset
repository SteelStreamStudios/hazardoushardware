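; Explosive barrel that pulses a material glow until a BP_Projectile hits it, then explodes with particles and a radial impulse on its Chaos component.
; A normal hit turns it red and explodes after a short delay; in one level this also updates the rubble, conveyor and divider actors.
; One level and type combination instead runs a cutscene, locking input, blending to BP_Camera and playing the Ramp sequence.
; Robot damage logic is unconnected.
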(event `self.ReceiveBeginPlay`
  (bind _chaos_explosivebarrel (`self.Chaos_ExplosiveBarrel`))
  (bind _asbp_game_state (cast `/Game/Blueprints/Class/BP_GameState` (`GameplayStatics.GetGameState`)))
  (set `self.As BP Game State` _asbp_game_state)
  (bind _asbp_robot (cast `/Game/Blueprints/Class/BP_Robot` (`GameplayStatics.GetPlayerPawn` 0)))
  (set `self.As BP Robot` _asbp_robot)
  (bind _returnvalue (`PrimitiveComponent.CreateDynamicMaterialInstance` _chaos_explosivebarrel 0 (`PrimitiveComponent.GetMaterial` _chaos_explosivebarrel 0) "None"))
  (set `self.Mat` _returnvalue)
  (`self.Pulse`))

(event `self.Capsule.OnComponentBeginOverlap`
  (params (OverlappedComponent :type "PrimitiveComponent Object Reference") (OtherActor :type "Actor Object Reference") (OtherComp :type "PrimitiveComponent Object Reference") (OtherBodyIndex :type Integer) (bFromSweep :type Boolean) (SweepResult :type "HitResult Structure (by ref)"))
  (cast `/Game/Blueprints/Class/BP_Projectile` OtherActor)
  (set `self.Shot?` true)
  (if (`|EnumEquality` (`/Game/Blueprints/Class/BP_GameState.Level` (`self.As BP Game State`)) "NewEnumerator0")
    (if (`|EnumEquality` (`self.Type`) "NewEnumerator1")
      (`/Engine/EditorBlueprintResources/StandardMacros.DoOnce` false
        (:`Completed`
          (`self.TriggerCutscene`)))
      (else
        (`/Engine/EditorBlueprintResources/StandardMacros.DoOnce` false
          (:`Completed`
            (`self.ChangeColor`)
            (`KismetSystemLibrary.Delay` 0.5)
            (`self.Explode`)))))
    (else
      (`/Engine/EditorBlueprintResources/StandardMacros.DoOnce` false
        (:`Completed`
          (`self.ChangeColor`)
          (`KismetSystemLibrary.Delay` 1.0)
          (`self.Explode`))))))

(event `Explode`
  (bind _returnvalue (`SceneComponent.K2_GetComponentLocation` (`self.Chaos_ExplosiveBarrel`)))
  ;[1 1 1 1 40] Explode
  (`ActorComponent.Deactivate` (`self.PS_FlameBurst_System`))
  (`ActorComponent.Activate` (`self.Explosion`) true)
  (`PhysicsObjectBlueprintLibrary.ApplyRadialImpulse` (`self.Chaos_ExplosiveBarrel`) _returnvalue 200.0 5000.0 "RIF_Constant")
  (`PrimitiveComponent.AddForceAtLocation` (`self.Chaos_ExplosiveBarrel`) (0.0 0.0 100.0) _returnvalue "None")
  (`GameplayStatics.SpawnSoundAtLocation` "/Game/Audio/Level2/BarrelExplosion/BarrelExplosion1.BarrelExplosion1" (`SceneComponent.K2_GetComponentLocation` (`self.Chaos_ExplosiveBarrel`)) (struct) 0.6 1.0 0.0 "/Game/Audio/FurnaceSoundAttenuation.FurnaceSoundAttenuation" null)
  (`SceneComponent.SetVisibility` (`self.Chaos_ExplosiveBarrel`) false false)
  (if (`|EnumEquality` (`/Game/Blueprints/Class/BP_GameState.Level` (`self.As BP Game State`)) "NewEnumerator1")
    (bind _returnvalue_2 (`GameplayStatics.GetActorOfClass` "/Game/Blueprints/Class/BP_ExplodableRubble.BP_ExplodableRubble_C"))
    (`/Game/Blueprints/Class/BP_ExplodableRubble.DestroyRubble` _returnvalue_2)
    (bind _returnvalue_3 (`GameplayStatics.GetActorOfClass` "/Game/Blueprints/Class/BP_ConveyorSpline.BP_ConveyorSpline_C"))
    (`/Game/Blueprints/Class/BP_ConveyorSpline.AddItem` _returnvalue_3)
    (`/Game/Blueprints/Class/BP_ConveyorSpline.PlayTimeline` _returnvalue_3)
    (bind _returnvalue_4 (`GameplayStatics.GetActorOfClass` "/Game/Blueprints/Class/BP_Divider.BP_Divider_C"))
    (`/Game/Blueprints/Class/BP_Divider.BarrelDestroyed` _returnvalue_4)
    (`KismetSystemLibrary.Delay` 2.0)
    (`self.K2_DestroyActor`)
    (else
      (`KismetSystemLibrary.Delay` 2.0)
      (`self.K2_DestroyActor`))))

(event `TriggerCutscene`
  (bind _returnvalue (`GameplayStatics.GetPlayerController` 0))
  (bind _returnvalue_2 (`SceneComponent.K2_GetComponentLocation` (`self.Chaos_ExplosiveBarrel`)))
  ;[1 1 1 1 40] Cutscene
  (`ActorComponent.Activate` (`self.PS_FlameBurst_System`) true)
  (bind _returnvalue_3 (`GameplayStatics.GetActorOfClass` "/Game/Blueprints/Class/BP_Camera.BP_Camera_C"))
  (`self.DisableInput` (`GameplayStatics.GetPlayerPawn` 0) _returnvalue)
  (`PlayerController.SetViewTargetWithBlend` _returnvalue _returnvalue_3 2.0 "VTBlend_Linear" 0.0 false)
  (`KismetSystemLibrary.Delay` 2.4)
  (`GeometryCollectionComponent.SetEnableDamageFromCollision` (`self.Chaos_ExplosiveBarrel`) true)
  (`ActorComponent.Deactivate` (`self.PS_FlameBurst_System`))
  (`ActorComponent.Activate` (`self.Explosion`) true)
  (`PhysicsObjectBlueprintLibrary.ApplyRadialImpulse` (`self.Chaos_ExplosiveBarrel`) _returnvalue_2 200.0 5000.0 "RIF_Constant")
  (`PrimitiveComponent.AddForceAtLocation` (`self.Chaos_ExplosiveBarrel`) (0.0 0.0 100.0) _returnvalue_2 "None")
  (`SceneComponent.SetVisibility` (`self.Chaos_ExplosiveBarrel`) false false)
  (bind (_outactor _returnvalue_4) (`LevelSequencePlayer.CreateLevelSequencePlayer` "/Game/Sequences/Ramp.Ramp"))
  (`MovieSceneSequencePlayer.Play` _returnvalue_4)
  (`KismetSystemLibrary.Delay` 2.0)
  (`PlayerController.SetViewTargetWithBlend` (`GameplayStatics.GetPlayerController` 0) (`GameplayStatics.GetPlayerPawn` 0) 2.0 "VTBlend_Linear" 0.0 false)
  (`KismetSystemLibrary.Delay` 2.0)
  (`self.EnableInput` (`GameplayStatics.GetPlayerPawn` 0) (`GameplayStatics.GetPlayerController` 0))
  (`self.K2_DestroyActor`))

(event `Pulse`
  (if (not (`self.Shot?`))
    (bind (_direction _newtrack_0) (`Timeline|Timeline` :!via `PlayFromStart`)
      (:`Update`
        (if (`self.Shot?`)
          (`MaterialInstanceDynamic.SetScalarParameterValue` (`self.Mat`) "Glow" 5.0)
          (else
            (`MaterialInstanceDynamic.SetScalarParameterValue` (`self.Mat`) "Glow" (`KismetMathLibrary.Lerp` 0.0 5.0 _newtrack_0)))))
      (:`Finished`
        (`self.Pulse`)))))

(event `ChangeColor`
  (`/Engine/EditorBlueprintResources/StandardMacros.DoOnce` false
    (:`Completed`
      (`MaterialInstanceDynamic.SetVectorParameterValue` (`self.Mat`) "Color" (struct :`R` 0.375 :`B` 0.009764 :`A` 1.0)))))

(fn `UserConstructionScript`)