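; BP_ScanningTurret is a turret that aims at the player's BP_Robot and fires at it, behind a shield that blocks projectiles.
; PawnSensing yaws the poseable mesh's base bone toward the robot's bullet spawn, then triggers Fire.
; Fire spawns three-shot BP_TurretProjectile bursts from the Arrow, repeating after a cooldown while Sensed remains set.
; Collider destroys incoming BP_Projectiles and flashes the shield sphere's material opacity through two timelines.
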(event `self.ReceiveBeginPlay`
  (bind _returnvalue (`PrimitiveComponent.CreateDynamicMaterialInstance` (`self.Sphere`) 0 (`PrimitiveComponent.GetMaterial` (`self.Sphere`) 0) "None"))
  (bind _output_get (set `self.Material` _returnvalue))
  (`MaterialInstanceDynamic.SetScalarParameterValue` _returnvalue "Opacity" (`self.Opacity`))
  (`MaterialInstanceDynamic.SetScalarParameterValue` _output_get "Opacity" (`self.Opacity`)))

(event `self.PawnSensing.OnSeePawn`
  (params (Pawn :type "Pawn Object Reference"))
  (set `self.Sensed` true)
  (bind _asbp_robot (cast `/Game/Blueprints/Class/BP_Robot` (`GameplayStatics.GetPlayerPawn` 0)))
  (bind _returnvalue (`PoseableMeshComponent.GetBoneRotationByName` (`self.PoseableMesh`) "Base_JNT" "ComponentSpace"))
  (bind (_returnvalue_roll _returnvalue_pitch _returnvalue_yaw) (`KismetMathLibrary.BreakRotator` (`KismetMathLibrary.FindLookAtRotation` (`self.K2_GetActorLocation`) (`SceneComponent.K2_GetComponentLocation` (`/Game/Blueprints/Class/BP_Robot.BulletSpawn` _asbp_robot)))))
  (`PoseableMeshComponent.SetBoneRotationByName` (`self.PoseableMesh`) "Base_JNT" (`KismetMathLibrary.MakeRotator` (.roll _returnvalue) (.pitch _returnvalue) (+ _returnvalue_yaw 180.0)) "WorldSpace")
  (`KismetSystemLibrary.Delay` 0.2)
  (if (`self.Firing?`)
    (set `self.Sensed` false)
    (else
      (`self.Fire`)
      (set `self.Sensed` false))))

(event `Fire`
  (bind _returnvalue (`SceneComponent.K2_GetComponentToWorld` (`self.Arrow`)))
  (if (not (`self.Firing?`))
    (set `self.Firing?` true)
    (`|SpawnActorFromClass` "/Game/Blueprints/Class/BP_TurretProjectile.BP_TurretProjectile_C" (`KismetMathLibrary.MakeTransform` (.location _returnvalue) (`KismetMathLibrary.MakeRotator` 0.0 0.0 (.yaw (.rotation _returnvalue)))) "Undefined" "MultiplyWithRoot" null null)
    (`KismetSystemLibrary.Delay` 0.1)
    (`|SpawnActorFromClass` "/Game/Blueprints/Class/BP_TurretProjectile.BP_TurretProjectile_C" (`KismetMathLibrary.MakeTransform` (.location _returnvalue) (`KismetMathLibrary.MakeRotator` 0.0 0.0 (.yaw (.rotation _returnvalue)))) "Undefined" "MultiplyWithRoot" null null)
    (`KismetSystemLibrary.Delay` 0.1)
    (`|SpawnActorFromClass` "/Game/Blueprints/Class/BP_TurretProjectile.BP_TurretProjectile_C" (`KismetMathLibrary.MakeTransform` (.location _returnvalue) (`KismetMathLibrary.MakeRotator` 0.0 0.0 (.yaw (.rotation _returnvalue)))) "Undefined" "MultiplyWithRoot" null null)
    (`KismetSystemLibrary.Delay` 2.0)
    (set `self.Firing?` false)
    (if (`self.Sensed`)
      (`self.Fire`))))

(event `self.Collider.OnComponentBeginOverlap`
  (params (OverlappedComponent :type "PrimitiveComponent Object Reference") (OtherActor :type "Actor Object Reference") (OtherComp :type "PrimitiveComponent Object Reference") (OtherBodyIndex :type Integer) (bFromSweep :type Boolean) (SweepResult :type "HitResult Structure (by ref)"))
  (bind _asbp_projectile (cast `/Game/Blueprints/Class/BP_Projectile` OtherActor))
  (`self.K2_DestroyActor` _asbp_projectile)
  (bind (_direction _newtrack_0) (`Timeline|ShowShield`)
    (:`Update`
      (`|ExecutionSequence`
        (:`then_0`
          (`MaterialInstanceDynamic.SetScalarParameterValue` (`self.Material`) "Opacity" (`KismetMathLibrary.Lerp` 0.0 1.0 _newtrack_0)))
        (:`then_1`
          (bind (_direction_2 _newtrack_0_2) (`Timeline|Timeline` :!via `Stop` :!label _label)
            (:`Update`
              (`MaterialInstanceDynamic.SetScalarParameterValue` (`self.Material`) "Opacity" (`KismetMathLibrary.Lerp` 1.0 0.0 _newtrack_0_2)))))))
    (:`Finished`
      (goto _label :!via `PlayFromStart`))))

(fn `UserConstructionScript`)