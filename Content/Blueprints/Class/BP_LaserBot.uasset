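; BP_LaserBot is a laser hazard that sweeps between two locations and damages the player's BP_Robot.
; Attack activates a Niagara beam, moves the actor out and back on timelines, then repeats while Lockdown is set.
; While firing, Tick traces downward to place the beam's end, and box overlaps deal damage with a one-second cooldown.
; A material glow event exists, but its only call sits in an unconnected waypoint-style chain.
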(event `StartGlow`
  (bind (_direction _time) (`Timeline|Start` :!via `PlayFromStart`)
    (:`Update`
      (`MaterialInstanceDynamic.SetScalarParameterValue` (`self.MaterialInstance`) "Glow" (`KismetMathLibrary.Lerp` 0.0 3.0 _time)))))

(event `self.ReceiveBeginPlay`
  (bind _returnvalue (`PrimitiveComponent.CreateDynamicMaterialInstance` (`self.Mesh`) 0 (`PrimitiveComponent.GetMaterial` (`self.Mesh`) 0) "None"))
  (set `self.MaterialInstance` _returnvalue)
  (`KismetSystemLibrary.Delay` 2.0))

(event `self.ReceiveTick`
  (params (DeltaSeconds :type "Float (single-precision)"))
  (bind (_returnvalue_x _returnvalue_y _returnvalue_z) (`KismetMathLibrary.BreakVector` (`SceneComponent.K2_GetComponentLocation` (`self.Mesh`))))
  (bind (_returnvalue_x_2 _returnvalue_y_2) (`KismetMathLibrary.BreakVector` (`SceneComponent.K2_GetComponentLocation` (`self.Mesh`))))
  (bind _returnvalue (`SceneComponent.K2_GetComponentLocation` (`self.Mesh`)))
  (if (`self.Firing`)
    (`FXSystemComponent.SetVectorParameter` (`self.NG_Beams`) "BeamStart" _returnvalue)
    (bind _outhit (`KismetSystemLibrary.LineTraceSingle` _returnvalue (`KismetMathLibrary.MakeVector` _returnvalue_x _returnvalue_y (- _returnvalue_z 1000.0)) "TraceTypeQuery4"))
    (`FXSystemComponent.SetVectorParameter` (`self.NG_Beams`) "BeamEnd" (`KismetMathLibrary.MakeVector` _returnvalue_x_2 _returnvalue_y_2 (.z (`.Location` (`GameplayStatics.BreakHitResult` _outhit)))))))

(event `Attack`
  (if (not (`self.Firing`))
    (set `self.Firing` true)
    (`ActorComponent.Activate` (`self.NG_Beams`) true)
    (`KismetSystemLibrary.Delay` 2.0)
    (bind (_direction _newtrack_0) (`Timeline|Sweep` :!via `PlayFromStart`)
      (:`Update`
        (`self.K2_SetActorLocation` (`KismetMathLibrary.VLerp` (`self.FirstLocation`) (`self.SecondLocation`) _newtrack_0)))
      (:`Finished`
        (`KismetSystemLibrary.Delay` 2.0)
        (bind (_direction_2 _newtrack_0_2) (`Timeline|Timeline` :!via `PlayFromStart`)
          (:`Update`
            (`self.K2_SetActorLocation` (`KismetMathLibrary.VLerp` (`self.SecondLocation`) (`self.FirstLocation`) _newtrack_0_2)))
          (:`Finished`
            (`KismetSystemLibrary.Delay` 2.0)
            (`ActorComponent.Deactivate` (`self.NG_Beams`))
            (set `self.Firing` false)
            (`KismetSystemLibrary.Delay` 5.0)
            (if (`self.Lockdown`)
              (`self.Attack`))))))))

(event `self.Box.OnComponentBeginOverlap`
  (params (OverlappedComponent :type "PrimitiveComponent Object Reference") (OtherActor :type "Actor Object Reference") (OtherComp :type "PrimitiveComponent Object Reference") (OtherBodyIndex :type Integer) (bFromSweep :type Boolean) (SweepResult :type "HitResult Structure (by ref)"))
  (bind _returnvalue (`GameplayStatics.GetPlayerPawn` 0))
  (if (== OtherActor _returnvalue)
    (if (`self.Firing`)
      (bind _asbp_robot (cast `/Game/Blueprints/Class/BP_Robot` _returnvalue))
      (`/Engine/EditorBlueprintResources/StandardMacros.DoOnce` false :!label _label
        (:`Completed`
          (`/Game/Blueprints/Class/BP_Robot.Damage` _asbp_robot)
          (`KismetSystemLibrary.Delay` 1.0)
          (goto _label :!via `Reset`))))))

(fn `UserConstructionScript`)