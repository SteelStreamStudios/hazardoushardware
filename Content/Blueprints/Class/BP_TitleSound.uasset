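; BP_TitleSound plays the title screen music as a three-part sequence: intro, activate and loop.
; On BeginPlay it casts player controller 0 to BP_PlayerController and plays the intro on its Audio component.
; Fixed delays time each switch to the next sound, which happens only while the controller's TitleScreenOn flag is still set.
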(event `self.ReceiveBeginPlay`
  (bind _audio (`self.Audio`))
  (bind _audio_2 (`self.Audio`))
  (bind _audio_3 (`self.Audio`))
  (bind _asbp_player_controller (cast `/Game/Blueprints/Class/BP_PlayerController` (`GameplayStatics.GetPlayerController` 0)))
  (set `self.As BP Player Controller` _asbp_player_controller)
  (`AudioComponent.SetSound` _audio_2 "/Game/UI/TitleCard/titlecardIntroAudio.titlecardIntroAudio")
  (`AudioComponent.Play` _audio_2 0.0)
  (`KismetSystemLibrary.Delay` 11.4)
  (if (`/Game/Blueprints/Class/BP_PlayerController.TitleScreenOn` (`self.As BP Player Controller`))
    (`AudioComponent.SetSound` _audio_3 "/Game/UI/TitleCard/titlecardActivateAudio.titlecardActivateAudio")
    (`AudioComponent.Play` _audio_3 0.0)
    (`KismetSystemLibrary.Delay` 35.0)
    (if (`/Game/Blueprints/Class/BP_PlayerController.TitleScreenOn` (`self.As BP Player Controller`))
      (`AudioComponent.SetSound` _audio "/Game/UI/TitleCard/titlecardLoopAudio.titlecardLoopAudio")
      (`AudioComponent.Play` _audio 0.0))))

(fn `UserConstructionScript`)