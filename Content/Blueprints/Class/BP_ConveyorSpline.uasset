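; Conveyor actor that carries explosive barrels along a spline, one at a time, in an endless loop.
; On BeginPlay it spawns a barrel and plays a timeline, rate-scaled by TimelineLength, that lerps distance along the spline to set the barrel's location and tangent-facing rotation.
; When the timeline finishes, it spawns the next barrel and restarts, leaving the previous one undestroyed.
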(event `self.ReceiveBeginPlay`
  (`self.AddItem`)
  (`self.PlayTimeline`))

(event `AddItem`
  (bind _returnvalue (`|SpawnActorFromClass` "/Game/Blueprints/Class/BP_ExplosiveBarrel.BP_ExplosiveBarrel_C" (`KismetMathLibrary.MakeTransform` (`SceneComponent.K2_GetComponentLocation` (`self.Spline`))) "Undefined" "MultiplyWithRoot" null null))
  (set `self.Actor` _returnvalue))

(event `PlayTimeline`
  (bind _actor (`self.Actor`))
  (`TimelineComponent.SetPlayRate` (`self.Timeline`) (/ 1.0 (`self.TimelineLength`)))
  (bind (_direction _newtrack_0) (`Timeline|Timeline` :!via `PlayFromStart`)
    (:`Update`
      (bind _returnvalue (`KismetMathLibrary.Lerp` 0.0 (`SplineComponent.GetDistanceAlongSplineAtSplinePoint` (`self.Spline`) (- (`SplineComponent.GetNumberOfSplinePoints` (`self.Spline`)) 1)) _newtrack_0))
      (`self.K2_SetActorLocation` _actor (`SplineComponent.GetLocationAtDistanceAlongSpline` (`self.Spline`) _returnvalue "World") false false)
      (`self.K2_SetActorRotation` _actor (`KismetMathLibrary.Conv_VectorToRotator` (`SplineComponent.GetTangentAtDistanceAlongSpline` (`self.Spline`) _returnvalue "World")) false))
    (:`Finished`
      (`self.AddItem`)
      (`self.PlayTimeline`))))

(fn `UserConstructionScript`
  (`self.K2_SetActorLocation` (`self.Actor`) (`SplineComponent.GetLocationAtSplinePoint` (`self.Spline`) 0 "Local") false false))