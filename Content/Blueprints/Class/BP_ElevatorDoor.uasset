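; Elevator door actor that plays open and close animations on its Door mesh.
; BeginPlay caches the BP_GameState and plays the open animation if the Open flag is set, leaving collision untouched.
; OpenDoor runs only once, playing the open animation and disabling collision on the Door and Cube.
; CloseDoor plays the close animation without restoring collision.
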(event `self.ReceiveBeginPlay`
  (bind _asbp_game_state (cast `/Game/Blueprints/Class/BP_GameState` (`GameplayStatics.GetGameState`)))
  (set `self.As BP Game State` _asbp_game_state)
  (if (`self.Open?`)
    (`SkeletalMeshComponent.PlayAnimation` (`self.Door`) "/Game/Meshes/Environment/A_ElevatorDoorOpen_Anim.A_ElevatorDoorOpen_Anim" false)))

(event `CloseDoor`
  (`SkeletalMeshComponent.PlayAnimation` (`self.Door`) "/Game/Animations/Props/A_ElevatorDoorClose_Anim.A_ElevatorDoorClose_Anim" false))

(event `OpenDoor`
  (`/Engine/EditorBlueprintResources/StandardMacros.DoOnce` false
    (:`Completed`
      (`SkeletalMeshComponent.PlayAnimation` (`self.Door`) "/Game/Meshes/Environment/A_ElevatorDoorOpen_Anim.A_ElevatorDoorOpen_Anim" false)
      (`PrimitiveComponent.SetCollisionEnabled` (`self.Door`) "NoCollision")
      (`PrimitiveComponent.SetCollisionEnabled` (`self.Cube`) "NoCollision"))))

(fn `UserConstructionScript`)