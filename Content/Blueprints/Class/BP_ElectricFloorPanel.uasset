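; Electric floor hazard panel that alternates between electrified and safe on a repeating timer, damaging the player's BP_Robot unless its full shield is up.
; Damage triggers on stepping onto a live panel, or standing on it when it switches on.
; Construction creates dynamic materials and sets the initial look from power and electrified flags.
; Each switch changes color and Niagara visibility, with a delayed timeline-driven glow blink during the safe phase.
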(event `Blink`
  (`KismetSystemLibrary.Delay` 1.0)
  (if (not (`self.Electrifed`))
    (bind (_direction _newtrack_0) (`Timeline|BlinkLight` :!via `PlayFromStart`)
      (:`Update`
        (`MaterialInstanceDynamic.SetScalarParameterValue` (`self.Array Element`) "Glow" (`KismetMathLibrary.Lerp` 0.0 2.0 _newtrack_0))))))

(event `self.ReceiveBeginPlay`
  (`self.Blink`)
  (`KismetSystemLibrary.Delay` 4.5)
  (`self.FloorSwitch` :!label _label)
  (if (not (`self.Electrifed`))
    (`self.Blink`))
  (`KismetSystemLibrary.RetriggerableDelay` 4.5)
  (goto _label))

(event `self.Box.OnComponentBeginOverlap`
  (params (OverlappedComponent :type "PrimitiveComponent Object Reference") (OtherActor :type "Actor Object Reference") (OtherComp :type "PrimitiveComponent Object Reference") (OtherBodyIndex :type Integer) (bFromSweep :type Boolean) (SweepResult :type "HitResult Structure (by ref)"))
  (bind _returnvalue (`GameplayStatics.GetPlayerPawn` 0))
  ;[1 1 1] Electrify Player
  (if (== OtherActor _returnvalue)
    (if (`self.Electrifed`)
      (bind _asbp_robot (cast `/Game/Blueprints/Class/BP_Robot` _returnvalue))
      (if (not (`/Game/Blueprints/Class/BP_Robot.FullShieldUP` _asbp_robot))
        (`/Game/Blueprints/Class/BP_Robot.Damage` _asbp_robot)))))

(event `FloorSwitch`
  (bind _returnvalue (`GameplayStatics.GetPlayerPawn` 0))
  (if (`self.Electrifed`)
    (`MaterialInstanceDynamic.SetVectorParameterValue` (`self.Array Element`) "Color" (struct :`R` 0.572917 :`B` 0.020254 :`A` 1.0))
    (set `self.Electrifed` false)
    (`SceneComponent.SetVisibility` (`self.Niagara`) false false)
    (else
      (`MaterialInstanceDynamic.SetVectorParameterValue` (`self.Array Element`) "Color" (struct :`G` 0.293571 :`B` 0.463542 :`A` 1.0))
      (set `self.Electrifed` true)
      (`SceneComponent.SetVisibility` (`self.Niagara`) true false)
      (if (`PrimitiveComponent.IsOverlappingActor` (`self.Box`) _returnvalue)
        (bind _asbp_robot (cast `/Game/Blueprints/Class/BP_Robot` _returnvalue))
        (if (not (`/Game/Blueprints/Class/BP_Robot.FullShieldUP` _asbp_robot))
          (`/Game/Blueprints/Class/BP_Robot.Damage` _asbp_robot))))))

(fn `UserConstructionScript`
  (bind _sm_electricfloor (`self.SM_ElectricFloor`))
  (for (_array_element _array_index) (`MeshComponent.GetMaterials` _sm_electricfloor)
    (bind _returnvalue (`PrimitiveComponent.CreateDynamicMaterialInstance` _sm_electricfloor _array_index _array_element "None"))
    (`KismetArrayLibrary.Array_Set` (`self.Target Array`) _array_index _returnvalue true))
  (for _array_element_2 (`self.Target Array`)
    (bind _output_get (set `self.Array Element` _array_element_2))
    (if (`self.PowerOn`)
      (if (`self.Electrifed`)
        (`MaterialInstanceDynamic.SetVectorParameterValue` _output_get "Color" (struct :`G` 0.300683 :`B` 0.630208 :`A` 1.0))
        (`MaterialInstanceDynamic.SetScalarParameterValue` _output_get "Glow" 2.0)
        (`SceneComponent.SetVisibility` (`self.Niagara`) true false)
        (else
          (`MaterialInstanceDynamic.SetVectorParameterValue` _output_get "Color" (struct :`R` 0.572917 :`B` 0.02531 :`A` 1.0))
          (`MaterialInstanceDynamic.SetScalarParameterValue` _output_get "Glow" 2.0)
          (`SceneComponent.SetVisibility` (`self.Niagara`) false false)))
      (else
        (`MaterialInstanceDynamic.SetScalarParameterValue` _output_get "Glow" 0.0)
        (`SceneComponent.SetVisibility` (`self.Niagara`) false false)))))