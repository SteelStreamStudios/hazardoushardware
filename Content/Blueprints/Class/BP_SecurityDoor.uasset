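; BP_SecurityDoor is a door that opens when the first player's pawn overlaps its trigger box and can be locked again through LockDoor.
; OpenDoor and LockDoor switch the Cube's collision and an Open flag, using paired DoOnce gates that reset each other.
; The overlap trigger fires only once, calling OpenDoor and playing controller vibration after a short delay.
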(event `LockDoor`
  (if (`self.Open`)
    (`/Engine/EditorBlueprintResources/StandardMacros.DoOnce` false :!label _label
      (:`Completed`
        (set `self.Open` false)
        (`PrimitiveComponent.SetCollisionEnabled` (`self.Cube`) "QueryAndPhysics")
        (goto _label_2 :!via `Reset`)))))

(event `OpenDoor`
  (if (not (`self.Open`))
    (`/Engine/EditorBlueprintResources/StandardMacros.DoOnce` false :!label _label_2
      (:`Completed`
        (set `self.Open` true)
        (`PrimitiveComponent.SetCollisionEnabled` (`self.Cube`) "NoCollision")
        (goto _label :!via `Reset`)))))

(event `self.Box.OnComponentBeginOverlap`
  (params (OverlappedComponent :type "PrimitiveComponent Object Reference") (OtherActor :type "Actor Object Reference") (OtherComp :type "PrimitiveComponent Object Reference") (OtherBodyIndex :type Integer) (bFromSweep :type Boolean) (SweepResult :type "HitResult Structure (by ref)"))
  (if (== OtherActor (`GameplayStatics.GetPlayerPawn` 0))
    (`/Engine/EditorBlueprintResources/StandardMacros.DoOnce` false
      (:`Completed`
        (`self.OpenDoor`)
        (`KismetSystemLibrary.Delay` 0.5)
        (`PlayerController.K2_ClientPlayForceFeedback` (`GameplayStatics.GetPlayerController` 0) "/Game/Misc/ForceFeedback/ControllerVibration.ControllerVibration" "None" false false false)))))

(fn `UserConstructionScript`)