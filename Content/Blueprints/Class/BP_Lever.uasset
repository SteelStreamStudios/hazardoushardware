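; BP_Lever is a one-shot lever that plays its pull animation, then after a short delay opens the BP_ElevatorDoor found by class lookup.
; Until it is pulled, player pawn overlap with its Box shows a widget and leaving hides it.
; Two Timelines scale the widget up and down, while paired DoOnce nodes re-arm each other so show and hide alternate.
; PullLever also hides the widget.
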(event `PullLever`
  (if (not (`self.LeverPulled`))
    (`SkeletalMeshComponent.PlayAnimation` (`self.Lever`) "/Game/Animations/Props/A_Mesh__Animationlever_Anim.A_Mesh__Animationlever_Anim" false)
    (`self.UIOff`)
    (set `self.LeverPulled` true)
    (`KismetSystemLibrary.Delay` 1.5)
    (bind _returnvalue (`GameplayStatics.GetActorOfClass` "/Game/Blueprints/Class/BP_ElevatorDoor.BP_ElevatorDoor_C"))
    (`/Game/Blueprints/Class/BP_ElevatorDoor.OpenDoor` _returnvalue)))

(event `self.Box.OnComponentBeginOverlap`
  (params (OverlappedComponent :type "PrimitiveComponent Object Reference") (OtherActor :type "Actor Object Reference") (OtherComp :type "PrimitiveComponent Object Reference") (OtherBodyIndex :type Integer) (bFromSweep :type Boolean) (SweepResult :type "HitResult Structure (by ref)"))
  (if (== OtherActor (`GameplayStatics.GetPlayerPawn` 0))
    (`/Engine/EditorBlueprintResources/StandardMacros.DoOnce` false :!label _label
      (:`Completed`
        (if (not (`self.LeverPulled`))
          (`self.UIOn`)
          (goto _label_2 :!via `Reset`))))))

(event `self.Box.OnComponentEndOverlap`
  (params (OverlappedComponent :type "PrimitiveComponent Object Reference") (OtherActor :type "Actor Object Reference") (OtherComp :type "PrimitiveComponent Object Reference") (OtherBodyIndex :type Integer))
  (if (== OtherActor (`GameplayStatics.GetPlayerPawn` 0))
    (`/Engine/EditorBlueprintResources/StandardMacros.DoOnce` true :!label _label_2
      (:`Completed`
        (if (not (`self.LeverPulled`))
          (`self.UIOff`)
          (goto _label :!via `Reset`))))))

(event `UIOn`
  (`/Engine/EditorBlueprintResources/StandardMacros.DoOnce` false :!label _label_3
    (:`Completed`
      (`|ExecutionSequence`
        (:`then_0`
          (bind (_direction _newtrack_0) (`Timeline|Timeline_0` :!via `Stop` :!label _label_4)
            (:`Update`
              (`SceneComponent.SetWorldScale3D` (`self.Widget`) (`KismetMathLibrary.VLerp` (0.6 0.6 0.6) (0.01 0.01 0.01) _newtrack_0)))))
        (:`then_1`
          (bind (_direction_2 _newtrack_0_2) (`Timeline|Timeline` :!via `PlayFromStart` :!label _label_5)
            (:`Update`
              (`SceneComponent.SetWorldScale3D` (`self.Widget`) (`KismetMathLibrary.VLerp` (0.01 0.01 0.01) (0.6 0.6 0.6) _newtrack_0_2)))))
        (:`then_2`
          (goto _label_6 :!via `Reset`))))))

(event `UIOff`
  (`/Engine/EditorBlueprintResources/StandardMacros.DoOnce` true :!label _label_6
    (:`Completed`
      (`|ExecutionSequence`
        (:`then_0`
          (goto _label_5 :!via `Stop`))
        (:`then_1`
          (goto _label_4 :!via `PlayFromStart`))
        (:`then_2`
          (goto _label_3 :!via `Reset`))))))

(fn `UserConstructionScript`)