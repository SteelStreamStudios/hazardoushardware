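; Pickup actor that grants the player robot one of four upgrades: plasma arm, gas wheel, shield arm or dash legs.
; PickUP branches on the item enum, sets the GameState flag, updates the robot and destroys itself.
; The plasma arm also opens a popup, shows the cursor and disables movement.
; Sphere overlaps drive paired timelines, gated by DoOnce nodes, that scale a "Press E" prompt plane in and out.
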(event `self.ReceiveBeginPlay`
  (bind _asbp_game_state (cast `/Game/Blueprints/Class/BP_GameState` (`GameplayStatics.GetGameState`)))
  (set `self.As BP Game State` _asbp_game_state)
  (bind _asbp_player_controller (cast `/Game/Blueprints/Class/BP_PlayerController` (`GameplayStatics.GetPlayerController` 0)))
  (set `self.As BP Player Controller` _asbp_player_controller))

(event `PickUP`
  (bind _as_bp_robot (`self.As BP Robot`))
  (bind _popupwidget (`/Game/Blueprints/Class/BP_PlayerController.PopUpWidget` (`self.As BP Player Controller`)))
  (bind _asbp_robot (cast `/Game/Blueprints/Class/BP_Robot` (`GameplayStatics.GetPlayerPawn` 0)))
  (set `self.As BP Robot` _asbp_robot)
  (if (`|EnumEquality` (`self.PickUpItem`) "NewEnumerator0")
    (set `/Game/Blueprints/Class/BP_GameState.HasPlasmaArm` true (`self.As BP Game State`))
    (`/Game/Blueprints/Class/BP_Robot.PlasmaArmEquip` (`self.As BP Robot`))
    (`SceneComponent.SetVisibility` (`self.PickUpMesh`) false false)
    (`UserWidget.AddToViewport` _popupwidget 0)
    (`/Game/Blueprints/UI/BP_PopUp_Widget.PlasmaOpen` _popupwidget)
    (`CharacterMovementComponent.DisableMovement` (`Character.CharacterMovement` (`GameplayStatics.GetPlayerCharacter` 0)))
    (set `PlayerController.bShowMouseCursor` true (`GameplayStatics.GetPlayerController` 0))
    (set `/Game/Blueprints/Class/BP_Robot.MaxMouseWheel` 1 (`self.As BP Robot`))
    (`self.K2_DestroyActor`)
    (elif (`|EnumEquality` (`self.PickUpItem`) "NewEnumerator1")
      (set `/Game/Blueprints/Class/BP_GameState.HasGasWheel` true (`self.As BP Game State`))
      (`SceneComponent.SetVisibility` (`/Game/Blueprints/Class/BP_Robot.BackItem` (`self.As BP Robot`)) true false)
      (`self.K2_DestroyActor`)
      (elif (`|EnumEquality` (`self.PickUpItem`) "NewEnumerator2")
        (set `/Game/Blueprints/Class/BP_GameState.HasShieldArm` true (`self.As BP Game State`))
        (set `/Game/Blueprints/Class/BP_Robot.ShieldArmEquipped` true _as_bp_robot)
        (`/Game/Blueprints/Class/BP_Robot.ShieldArmEquip` _as_bp_robot)
        (set `/Game/Blueprints/Class/BP_Robot.MaxMouseWheel` 2 (`self.As BP Robot`))
        (`KismetSystemLibrary.Delay` 0.2)
        (`self.K2_DestroyActor`)
        (elif (`|EnumEquality` (`self.PickUpItem`) "NewEnumerator3")
          (set `/Game/Blueprints/Class/BP_GameState.HasDashLegs` true (`self.As BP Game State`))
          (`/Game/Blueprints/Class/BP_Robot.DashEquip` (`self.As BP Robot`))
          (set `/Game/Blueprints/Class/BP_Robot.MaxMouseWheel` 3 (`self.As BP Robot`))
          (`KismetSystemLibrary.Delay` 0.2)
          (`self.K2_DestroyActor`))))))

(event `self.Sphere.OnComponentBeginOverlap`
  (params (OverlappedComponent :type "PrimitiveComponent Object Reference") (OtherActor :type "Actor Object Reference") (OtherComp :type "PrimitiveComponent Object Reference") (OtherBodyIndex :type Integer) (bFromSweep :type Boolean) (SweepResult :type "HitResult Structure (by ref)"))
  ;[1 1 1] "Press E" Prompt Active
  (if (== OtherActor (`GameplayStatics.GetPlayerPawn` 0))
    (`/Engine/EditorBlueprintResources/StandardMacros.DoOnce` false :!label _label
      (:`Completed`
        (`|ExecutionSequence`
          (:`then_0`
            (bind (_direction _time) (`Timeline|Timeline` :!via `PlayFromStart` :!label _label_2)
              (:`Update`
                (`SceneComponent.SetWorldScale3D` (`self.Plane`) (`KismetMathLibrary.VLerp` (`SceneComponent.K2_GetComponentScale` (`self.Plane`)) (2.8 2.8 2.8) _time)))))
          (:`then_1`
            ;[1 1 1] "Press E" Prompt Deactive
            (bind (_direction_2 _time_2) (`Timeline|Timeline_0` :!via `Stop` :!label _label_3)
              (:`Update`
                (`SceneComponent.SetWorldScale3D` (`self.Plane`) (`KismetMathLibrary.VLerp` (`SceneComponent.K2_GetComponentScale` (`self.Plane`)) (0.0 0.0 0.0) _time_2)))))
          (:`then_2`
            (goto _label_4 :!via `Reset`)))))))

(event `self.Sphere.OnComponentEndOverlap`
  (params (OverlappedComponent :type "PrimitiveComponent Object Reference") (OtherActor :type "Actor Object Reference") (OtherComp :type "PrimitiveComponent Object Reference") (OtherBodyIndex :type Integer))
  ;[1 1 1] "Press E" Prompt Deactive
  (if (== OtherActor (`GameplayStatics.GetPlayerPawn` 0))
    (`/Engine/EditorBlueprintResources/StandardMacros.DoOnce` true :!label _label_4
      (:`Completed`
        (`|ExecutionSequence`
          (:`then_0`
            (goto _label_2 :!via `Stop`))
          (:`then_1`
            (goto _label_3 :!via `PlayFromStart`))
          (:`then_2`
            (goto _label :!via `Reset`)))))))

(fn `UserConstructionScript`)