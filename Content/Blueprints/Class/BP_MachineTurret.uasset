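; Shielded turret that powers up, rises through a level sequence and fires repeating three-shot projectile volleys from three arrows.
; PowerUp runs once, ramping Power and the glow on dynamic materials, then enables the shield collider.
; Fire applies an initial delay on the first shot, then re-calls itself after each staggered volley.
; The collider destroys overlapping BP_Projectile actors, flashing the shield sphere's opacity through fade-in and fade-out timelines.
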(event `self.ReceiveBeginPlay`
  (bind _turret (`self.Turret`))
  (for (_array_element _array_index) (`MeshComponent.GetMaterials` _turret)
    (bind _returnvalue (`PrimitiveComponent.CreateDynamicMaterialInstance` _turret _array_index _array_element "None"))
    (`KismetArrayLibrary.Array_Set` (`self.Target Array`) _array_index _returnvalue true))
  (`self.SetValues`)
  (bind _asbp_robot (cast `/Game/Blueprints/Class/BP_Robot` (`GameplayStatics.GetPlayerPawn` 0)))
  (set `self.As BP Robot` _asbp_robot)
  (bind _returnvalue_2 (`PrimitiveComponent.CreateDynamicMaterialInstance` (`self.Sphere`) 0 (`PrimitiveComponent.GetMaterial` (`self.Sphere`) 0) "None"))
  (bind _output_get (set `self.Material` _returnvalue_2))
  (`MaterialInstanceDynamic.SetScalarParameterValue` _output_get "Opacity" (`self.Value`))
  (`PrimitiveComponent.SetCollisionEnabled` (`self.Collider`) "NoCollision"))

(event `SetValues`
  (for _array_element (`self.Target Array`)
    (`MaterialInstanceDynamic.SetScalarParameterValue` _array_element "Glow" (`self.Glow`))
    (`MaterialInstanceDynamic.SetVectorParameterValue` _array_element "Color" (`self.Color`))))

(event `PowerUp`
  (`/Engine/EditorBlueprintResources/StandardMacros.DoOnce` false
    (:`Completed`
      (bind (_direction _newtrack_0) (`Timeline|Timeline`)
        (:`Update`
          (set `self.Power` (`KismetMathLibrary.Lerp` 0.0 100.0 _newtrack_0))
          (for _array_element (`self.Target Array`)
            (`MaterialInstanceDynamic.SetScalarParameterValue` _array_element "Glow" (`KismetMathLibrary.Lerp` 0.0 3.0 _newtrack_0))))
        (:`Finished`
          (`PrimitiveComponent.SetCollisionEnabled` (`self.Collider`) "QueryOnly"))))))

(event `RaiseTurret`
  (bind (_outactor _returnvalue) (`LevelSequencePlayer.CreateLevelSequencePlayer` "/Game/Sequences/RaiseTurrets.RaiseTurrets"))
  (`MovieSceneSequencePlayer.Play` _returnvalue))

(event `Fire`
  (bind (_returnvalue_location _returnvalue_rotation) (`KismetMathLibrary.BreakTransform` (`SceneComponent.K2_GetComponentToWorld` (`self.Arrow1`))))
  (bind (_returnvalue_location_2 _returnvalue_rotation_2) (`KismetMathLibrary.BreakTransform` (`SceneComponent.K2_GetComponentToWorld` (`self.Arrow2`))))
  (bind (_returnvalue_location_3 _returnvalue_rotation_3) (`KismetMathLibrary.BreakTransform` (`SceneComponent.K2_GetComponentToWorld` (`self.Arrow`))))
  (if (`self.FirstShot`)
    (`KismetSystemLibrary.Delay` (`self.Delay`))
    (set `self.FirstShot` false))
  (if (not (`self.Firing?`))
    (set `self.Firing?` true)
    (`SkeletalMeshComponent.PlayAnimation` (`self.Turret`) "/Game/Animations/Props/A_Fire_Anim.A_Fire_Anim" false)
    (`GameplayStatics.PlaySoundAtLocation` "/Game/Audio/Level2/TurretFireSoundCue.TurretFireSoundCue" _returnvalue_location_3 (struct) 0.6 1.0 0.0 "/Game/Audio/ConveyorAttenuation.ConveyorAttenuation" null null null)
    (`|SpawnActorFromClass` "/Game/Blueprints/Class/BP_TurretProjectile.BP_TurretProjectile_C" (`KismetMathLibrary.MakeTransform` _returnvalue_location_3 _returnvalue_rotation_3) "Undefined" "MultiplyWithRoot" null null)
    (`KismetSystemLibrary.Delay` 0.1)
    (`|SpawnActorFromClass` "/Game/Blueprints/Class/BP_TurretProjectile.BP_TurretProjectile_C" (`KismetMathLibrary.MakeTransform` _returnvalue_location _returnvalue_rotation) "Undefined" "MultiplyWithRoot" null null)
    (`KismetSystemLibrary.Delay` 0.1)
    (`|SpawnActorFromClass` "/Game/Blueprints/Class/BP_TurretProjectile.BP_TurretProjectile_C" (`KismetMathLibrary.MakeTransform` _returnvalue_location_2 _returnvalue_rotation_2) "Undefined" "MultiplyWithRoot" null null)
    (set `self.Firing?` false)
    (`KismetSystemLibrary.Delay` 2.0)
    (`self.Fire`)))

(event `self.Collider.OnComponentBeginOverlap`
  (params (OverlappedComponent :type "PrimitiveComponent Object Reference") (OtherActor :type "Actor Object Reference") (OtherComp :type "PrimitiveComponent Object Reference") (OtherBodyIndex :type Integer) (bFromSweep :type Boolean) (SweepResult :type "HitResult Structure (by ref)"))
  (bind _asbp_projectile (cast `/Game/Blueprints/Class/BP_Projectile` OtherActor))
  (`self.K2_DestroyActor` _asbp_projectile)
  (`GameplayStatics.PlaySoundAtLocation` "/Game/Audio/Level2/ShieldImpactSoundCue.ShieldImpactSoundCue" (`SceneComponent.K2_GetComponentLocation` (`self.Turret`)) (struct) 0.5 1.0 0.0 "/Game/Audio/FurnaceSoundAttenuation.FurnaceSoundAttenuation" null null null)
  (bind (_direction _newtrack_0) (`Timeline|Timeline_0`)
    (:`Update`
      (`|ExecutionSequence`
        (:`then_0`
          (`MaterialInstanceDynamic.SetScalarParameterValue` (`self.Material`) "Opacity" (`KismetMathLibrary.Lerp` 0.0 1.0 _newtrack_0)))
        (:`then_1`
          (bind (_direction_2 _newtrack_0_2) (`Timeline|Timeline_1` :!via `Stop` :!label _label)
            (:`Update`
              (`MaterialInstanceDynamic.SetScalarParameterValue` (`self.Material`) "Opacity" (`KismetMathLibrary.Lerp` 1.0 0.0 _newtrack_0_2)))))))
    (:`Finished`
      (goto _label :!via `PlayFromStart`))))

(fn `UserConstructionScript`)