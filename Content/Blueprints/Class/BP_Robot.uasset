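; Player robot character with fixed-axis movement, jump, flashlight, interaction trace, physics grab, scaling shield and a swappable plasma arm.
; Plasma shots and dashing drain a shared Charge that recharges after a delay, with overheating when empty.
; While armed, Tick traces the laser sight's length and outlines assembly arms and destructibles.
; Lost health or an unblocked missile strike triggers ragdoll disassembly, then destruction asks the GameMode to respawn.
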(event `EnhancedInput|/Game/Misc/Inputs/IA_Move`
  (params (ActionValue :type "Vector2D Structure") (ElapsedSeconds :type "Float (double-precision)") (TriggeredSeconds :type "Float (double-precision)") (InputAction :type "InputAction Object Reference" :default "/Game/Misc/Inputs/IA_Move.IA_Move"))
  ;[1 1 1 1 40] Movement
  (:`Triggered`
    (set `self.ForwardAxis` ActionValue_X)
    (set `self.Left/RightAxis` ActionValue_Y)
    (`self.AddMovementInput` (-1.0 1.0 0.0) (`self.ForwardAxis`))
    (`self.AddMovementInput` (1.0 1.0 0.0) (`self.Left/RightAxis`))))

(event `EarsOnMesh`
  (`PlayerController.SetAudioListenerOverride` :`self` (`GameplayStatics.GetPlayerController` 0) :`AttachToComponent` (`self.Mesh`)))

(event `EnhancedInput|/Game/Misc/Inputs/IA_Shoot`
  (params (ActionValue :type Boolean) (ElapsedSeconds :type "Float (double-precision)") (TriggeredSeconds :type "Float (double-precision)") (InputAction :type "InputAction Object Reference" :default "/Game/Misc/Inputs/IA_Shoot.IA_Shoot"))
  (bind (_returnvalue_location _returnvalue_rotation) (`KismetMathLibrary.BreakTransform` (`SceneComponent.K2_GetComponentToWorld` (`self.BulletSpawn`))))
  (:`Triggered`
    (if (`self.GunEquipped`) :!label _label
      (if (not (`self.Overheated`))
        (set `self.Shooting?` true)
        (`SceneComponent.SetVisibility` (`self.LaserSight`) false false)
        (if (> (`self.Charge`) 0.0)
          (`KismetSystemLibrary.Delay` 0.1)
          (`|ExecutionSequence`
            (:`then_0`
              (`|SpawnActorFromClass` "/Game/Blueprints/Class/BP_Projectile.BP_Projectile_C" (`KismetMathLibrary.MakeTransform` _returnvalue_location _returnvalue_rotation) "Undefined" "MultiplyWithRoot" null null)
              (`GameplayStatics.PlaySoundAtLocation` "/Game/Audio/PlasmaShot.PlasmaShot" _returnvalue_location (struct) 0.5 1.0 0.0 "/Game/Audio/FurnaceSoundAttenuation.FurnaceSoundAttenuation" null null null))
            (:`then_1`
              (`KismetSystemLibrary.Delay` 0.2)
              (`self.DecreaseCharge`)))
          (else
            (set `self.Shooting?` false)
            (set `self.Overheated` true))))))
  (:`Started`
    (goto _label))
  (:`Canceled`
    (if (`self.GunEquipped`) :!label _label_2
      (set `self.Shooting?` false)
      (`SceneComponent.SetVisibility` (`self.LaserSight`) true false)
      (`KismetSystemLibrary.Delay` 3.0)
      (`self.IncreaseCharge`)))
  (:`Completed`
    (goto _label_2)))

(event `/Game/Blueprints/Interfaces/BP_RobotInterface.Rotate`
  (params (Rotate :type "Rotator Structure"))
  (bind (_relativerotation_roll _relativerotation_pitch _relativerotation_yaw) (`KismetMathLibrary.BreakRotator` (`SceneComponent.RelativeRotation` (`self.SpringArm`))))
  ;[1 1 1 1 40] Movement
  (`self.K2_SetActorRotation` (`KismetMathLibrary.MakeRotator` 0.0 0.0 (- Rotate_Yaw _relativerotation_yaw))))

(event `EarsOnCamera`
  (`PlayerController.SetAudioListenerOverride` :`self` (`GameplayStatics.GetPlayerController` 0) :`AttachToComponent` (`self.Camera`)))

(event `EnhancedInput|/Game/Misc/Inputs/IA_Jump`
  (params (ActionValue :type Boolean) (ElapsedSeconds :type "Float (double-precision)") (TriggeredSeconds :type "Float (double-precision)") (InputAction :type "InputAction Object Reference" :default "/Game/Misc/Inputs/IA_Jump.IA_Jump"))
  ;[1 1 1 1 30] SPACE
  (:`Triggered`
    (`self.Jump` :!label _label_3))
  (:`Started`
    (goto _label_3))
  (:`Canceled`
    (`self.StopJumping` :!label _label_4))
  (:`Completed`
    (goto _label_4)))

(event `self.ReceiveBeginPlay`
  (bind _mesh (`self.Mesh`))
  ;[1 1 1 1 30] Begin Play
  (bind _asbp_player_controller (cast `/Game/Blueprints/Class/BP_PlayerController` (`GameplayStatics.GetPlayerController` 0)))
  (set `self.As Player Controller BP` _asbp_player_controller)
  (bind _asbp_game_state (cast `/Game/Blueprints/Class/BP_GameState` (`GameplayStatics.GetGameState`)))
  (set `self.As BP Game State` _asbp_game_state)
  (set `self.CurrentHealth` (`self.MaxHealth`))
  (bind _returnvalue (`PrimitiveComponent.CreateDynamicMaterialInstance` _mesh 0 (`PrimitiveComponent.GetMaterial` _mesh 0) "None"))
  (set `self.BodyMatInst` _returnvalue)
  (`PlayerController.SetAudioListenerOverride` :`self` (`GameplayStatics.GetPlayerController` 0) :`AttachToComponent` (`self.Mesh`)))

(event `DeployShield`
  (bind _sphere (`self.Sphere`))
  ;[1 1 1 1 40] Shield Ability
  (`/Engine/EditorBlueprintResources/StandardMacros.DoOnce` false :!label _label_5
    (:`Completed`
      (`|ExecutionSequence`
        (:`then_0`
          (bind (_direction _newtrack_0) (`Timeline|Timeline_0` :!via `Stop` :!label _label_6)
            (:`Update`
              (`SceneComponent.SetWorldScale3D` _sphere (`KismetMathLibrary.VLerp` (`SceneComponent.K2_GetComponentScale` _sphere) (0.0 0.0 0.0) _newtrack_0)))
            (:`Finished`
              (set `self.ShieldUp` false)
              (goto _label_5 :!via `Reset`))))
        (:`then_1`
          (bind (_direction_2 _newtrack_0_2) (`Timeline|Timeline` :!via `PlayFromStart` :!label _label_7)
            (:`Update`
              (`SceneComponent.SetWorldScale3D` (`self.Sphere`) (`KismetMathLibrary.VLerp` (`SceneComponent.K2_GetComponentScale` (`self.Sphere`)) (2.3 2.3 2.3) _newtrack_0_2)))
            (:`Finished`
              (set `self.ShieldUp` true)
              (goto _label_8 :!via `Reset`))))))))

(event `Key|E`
  (params (Key :type "Key Structure"))
  (bind _arrow1 (`self.Arrow1`))
  (bind _returnvalue (+ (`SceneComponent.K2_GetComponentLocation` _arrow1) (* (`SceneComponent.GetForwardVector` _arrow1) 100.0)))
  ;[1 1 1 1 40] Press E
  (:`Pressed`
    (bind (_outhit _returnvalue_2) (`KismetSystemLibrary.BoxTraceSingle` _returnvalue _returnvalue (80.0 80.0 100.0) (`SceneComponent.K2_GetComponentRotation` _arrow1) "TraceTypeQuery3"))
    (if _returnvalue_2
      (bind (_bblockinghit _binitialoverlap _time _distance _location _impactpoint _normal _impactnormal _physmat _hitactor) (`GameplayStatics.BreakHitResult` _outhit))
      (bind _asbp_audio_log (cast `/Game/Blueprints/Class/BP_AudioLog` _hitactor)
        (:`then`
          (`/Game/Blueprints/Interfaces/BP_PickUpInterface.PickUp` _asbp_audio_log))
        (:`CastFailed`
          (bind _asbp_electrical_switch (cast `/Game/Blueprints/Class/BP_ElectricalSwitch` _hitactor)
            (:`then`
              (`/Game/Blueprints/Class/BP_ElectricalSwitch.PowerOn` _asbp_electrical_switch))
            (:`CastFailed`
              (bind _asbp_flame_hazard (cast `/Game/Blueprints/Class/BP_FlameHazard` _hitactor)
                (:`then`
                  (`/Game/Blueprints/Class/BP_FlameHazard.TurnOff` _asbp_flame_hazard))
                (:`CastFailed`
                  (bind _asbp_pick_up (cast `/Game/Blueprints/Class/BP_PickUp` _hitactor))
                  (`/Game/Blueprints/Class/BP_PickUp.PickUP` _asbp_pick_up))))))))))

(event `RemoveShield`
  ;[1 1 1 1 40] Shield Ability
  (`/Engine/EditorBlueprintResources/StandardMacros.DoOnce` false :!label _label_8
    (:`Completed`
      (`|ExecutionSequence`
        (:`then_0`
          (goto _label_7 :!via `Stop`))
        (:`then_1`
          (goto _label_6 :!via `PlayFromStart`))))))

(event `DecreaseCharge`
  ;[1 1 1 1 45] Charge
  (if (> (`self.Charge`) 0.0)
    (if (`self.Shooting?`)
      (set `self.Charge` (- (`self.Charge`) 5.0)))))

(event `IncreaseCharge`
  ;[1 1 1 1 45] Charge
  (if (< (`self.Charge`) 100.0) :!label _label_9
    (if (>= (`self.Charge`) 50.0)
      (set `self.Overheated` false))
    (if (`self.Shooting?`)
      _
      (elif (not (`self.Dashing`))
        (set `self.Charge` (+ (`self.Charge`) 5.0))
        (`KismetSystemLibrary.RetriggerableDelay` 0.2)
        (goto _label_9)))))

(event `MissileStrike`
  ;[1 1 1 1 40] Missile Strike (QTE)
  (if (not (`self.Targeting`))
    (set `self.Targeting` true)
    (bind _returnvalue (`|SpawnActorFromClass` "/Game/Blueprints/Class/BP_MissileTarget.BP_MissileTarget_C" (`KismetMathLibrary.MakeTransform` (`SceneComponent.K2_GetComponentLocation` (`self.MissileTargetLocation`))) "Undefined" "MultiplyWithRoot" null null))
    (`self.K2_AttachToActor` _returnvalue self "Multibot_Center_Spine_JNT" "KeepWorld" "KeepWorld" "KeepWorld" true)
    (`/Game/Blueprints/Class/BP_MissileTarget.StartTarget` _returnvalue)
    (`KismetSystemLibrary.Delay` 3.0)
    (if (`/Game/Blueprints/Class/BP_MissileTarget.BlockMissile` _returnvalue)
      (set `self.Targeting` false)
      (else
        (set `self.Targeting` false)
        (`self.Disassemble`)
        (`PrimitiveComponent.AddImpulse` (`self.Mesh`) (0.0 0.0 10000.0) "None" false)
        (`PrimitiveComponent.AddImpulse` (`self.RightArm`) (0.0 0.0 10000.0) "None" false)
        (`PrimitiveComponent.AddImpulse` (`self.Legs`) (0.0 0.0 10000.0) "None" false)
        (`PrimitiveComponent.AddImpulse` (`self.LeftArm`) (0.0 0.0 10000.0) "None" false)))))

(event `ArmEquip`
  ;[1 1 1 1 40] Arm Switch
  (if (`self.GunEquipped`)
    (set `self.GunEquipped` false)
    (set `self.bUseControllerRotationYaw` false)
    (set `CharacterMovementComponent.bOrientRotationToMovement` true (`self.CharacterMovement`))
    (`SceneComponent.SetVisibility` (`self.LaserSight`) false false)
    (`SkeletalMeshComponent.SetSkeletalMeshAsset` (`self.RightArm`) "/Game/Meshes/Characters/SK_RobotRightArm.SK_RobotRightArm")
    (`SceneComponent.SetVisibility` (`self.Ammo`) false false)
    (`SceneComponent.SetVisibility` (`self.Crossair`) false false)
    (set `CharacterMovementComponent.JumpZVelocity` 400.0 (`self.CharacterMovement`))
    (else
      (set `self.GunEquipped` true)
      (set `self.bUseControllerRotationYaw` false)
      (set `CharacterMovementComponent.bOrientRotationToMovement` true (`self.CharacterMovement`))
      (`SceneComponent.SetVisibility` (`self.LaserSight`) true false)
      (`SkeletalMeshComponent.SetSkeletalMeshAsset` (`self.RightArm`) "/Game/Meshes/Characters/SK_PlasmaArm.SK_PlasmaArm")
      (`SceneComponent.SetVisibility` (`self.Ammo`) true false)
      (`SceneComponent.SetVisibility` (`self.Crossair`) false false)
      (set `CharacterMovementComponent.JumpZVelocity` 0.0 (`self.CharacterMovement`)))))

(event `Key|Q`
  (params (Key :type "Key Structure"))
  ;[1 1 1 1 40] Arm Switch
  (:`Pressed`
    (if (`/Game/Blueprints/Class/BP_GameState.HasPlasmaArm` (`self.As BP Game State`))
      (`self.ArmEquip`))))

(event `/Game/Blueprints/Interfaces/BP_RobotInterface.LookAt`
  (params (Target :type "Vector Structure"))
  (bind (_returnvalue_x _returnvalue_y _returnvalue_z) (`KismetMathLibrary.BreakVector` (`self.K2_GetActorLocation`)))
  ;[1 1 1 1 30] Player Rotation (For Plasma Arm)
  (`SceneComponent.K2_SetWorldRotation` (`self.BulletSpawn`) (`KismetMathLibrary.FindLookAtRotation` (`KismetMathLibrary.MakeVector` _returnvalue_x _returnvalue_y _returnvalue_z) (`KismetMathLibrary.MakeVector` Target_X Target_Y Target_Z)) false false)
  (`self.K2_SetActorRotation` (`KismetMathLibrary.FindLookAtRotation` (`KismetMathLibrary.MakeVector` _returnvalue_x _returnvalue_y) (`KismetMathLibrary.MakeVector` Target_X Target_Y))))

(event `self.ReceiveTick`
  (params (DeltaSeconds :type "Float (single-precision)"))
  ;[1 1 1 1 40] Event Tick
  (if (`self.GunEquipped`)
    (`self.SetLaserLength`)))

(event `Drop`
  ;[1 1 1 1 40] Pick Up Ability
  (`PhysicsHandleComponent.ReleaseComponent` (`self.PhysicsHandle`))
  (set `self.IsGrabbing` false))

(event `Lift`
  (bind _arrow1 (`self.Arrow1`))
  (bind _returnvalue (`SceneComponent.K2_GetComponentLocation` _arrow1))
  ;[1 1 1 1 40] Pick Up Ability
  (bind (_outhit _returnvalue_2) (`KismetSystemLibrary.CapsuleTraceSingle` _returnvalue (+ _returnvalue (* (`KismetMathLibrary.GetForwardVector` (`SceneComponent.K2_GetComponentRotation` _arrow1)) 100.0)) 40.0 80.0 "TraceTypeQuery1"))
  (if _returnvalue_2
    (bind (_bblockinghit _binitialoverlap _time _distance _location _impactpoint _normal _impactnormal _physmat _hitactor _hitcomponent) (`GameplayStatics.BreakHitResult` _outhit))
    (`PhysicsHandleComponent.GrabComponentAtLocationWithRotation` :`self` (`self.PhysicsHandle`) :`Component` _hitcomponent :`Location` (`SceneComponent.K2_GetComponentLocation` _hitcomponent))
    (set `self.IsGrabbing` true)))

(event `Key|RightMouseButton`
  (params (Key :type "Key Structure"))
  ;[1 1 1 1 40] Pick Up Ability
  (:`Pressed`
    (`self.Lift`))
  (:`Released`
    (if (`self.IsGrabbing`)
      (`self.Drop`))))

(event `Disassemble`
  ;[1 1 1 1 40] Death
  (`PrimitiveComponent.SetCollisionEnabled` (`self.CapsuleComponent`) "QueryAndPhysics")
  (set `self.Dead` true)
  (`PrimitiveComponent.SetCollisionProfileName` (`self.Mesh`) "Ragdoll" true)
  (`CharacterMovementComponent.DisableMovement` (`self.CharacterMovement`))
  (`PrimitiveComponent.SetSimulatePhysics` (`self.RightArm`) true)
  (`PrimitiveComponent.SetSimulatePhysics` (`self.Legs`) true)
  (`PrimitiveComponent.SetSimulatePhysics` (`self.LeftArm`) true)
  (`PrimitiveComponent.SetSimulatePhysics` (`self.Mesh`) true)
  (`SceneComponent.SetVisibility` (`self.Ammo`) false false)
  (`SceneComponent.SetVisibility` (`self.Crossair`) false false)
  (`KismetSystemLibrary.Delay` 3.0)
  (set `self.Dead` false)
  (`self.K2_DestroyActor`))

(event `self.ReceiveDestroyed`
  ;[1 1 1 1 40] Death
  (bind _asbp_hazardous_hardware_game_mode (cast `/Game/Blueprints/Class/BP_HazardousHardware_GameMode` (`GameplayStatics.GetGameMode`)))
  (`/Game/Blueprints/Class/BP_HazardousHardware_GameMode.Respawn` _asbp_hazardous_hardware_game_mode))

(event `Key|LeftShift`
  (params (Key :type "Key Structure"))
  ;[1 1 1 1 40] Dash
  (:`Pressed`
    (if (`self.DashLegEquipped`)
      (if (`self.Dashing`)
        _
        (elif (>= (`self.Charge`) 50.0)
          (`self.NewDash`))))))

(event `NewDash`
  (bind _charactermovement (`self.CharacterMovement`))
  ;[1 1 1 1 40] Dash
  (set `self.Dashing` true)
  (set `self.Charge` (- (`self.Charge`) 50.0))
  (set `CharacterMovementComponent.MaxWalkSpeed` 8000.0 _charactermovement)
  (set `CharacterMovementComponent.MaxAcceleration` 8000.0 _charactermovement)
  (set `CharacterMovementComponent.BrakingFriction` 3000.0 _charactermovement)
  (`KismetSystemLibrary.K2_SetTimerDelegate` (delegate `StopDashing`) 0.25))

(event `FlashlightToggle`
  ;[1 1 1] Flashlight
  (`/Engine/EditorBlueprintResources/StandardMacros.FlipFlop`
    (:`A`
      (`SceneComponent.SetVisibility` (`self.SpotLight`) true false)
      (`MaterialInstanceDynamic.SetScalarParameterValue` (`self.BodyMatInst`) "Glow" 10.0)
      (set `self.FlashlightOn` true)
      (`GameplayStatics.PlaySound2D` "/Engine/VREditor/Sounds/UI/Enter_Play.Enter_Play" 1.0 1.0 0.0 null null))
    (:`B`
      (`SceneComponent.SetVisibility` (`self.SpotLight`) false false)
      (`MaterialInstanceDynamic.SetScalarParameterValue` (`self.BodyMatInst`) "Glow" 0.0)
      (set `self.FlashlightOn` false)
      (`GameplayStatics.PlaySound2D` "/Engine/VREditor/Sounds/UI/Flashlight_Switch.Flashlight_Switch" 1.0 1.0 0.0 null null))))

(event `StopDashing`
  (bind _charactermovement (`self.CharacterMovement`))
  ;[1 1 1 1 40] Dash
  (set `CharacterMovementComponent.MaxWalkSpeed` 250.0 _charactermovement)
  (set `CharacterMovementComponent.MaxAcceleration` 1000.0 _charactermovement)
  (`KismetSystemLibrary.K2_SetTimerDelegate` (delegate `ResetBraking`) 0.2)
  (set `self.Dashing` false)
  (`KismetSystemLibrary.Delay` 3.0)
  (`self.IncreaseCharge`))

(event `Key|F`
  (params (Key :type "Key Structure"))
  ;[1 1 1] Flashlight
  (:`Pressed`
    (`self.FlashlightToggle`)))

(event `ResetBraking`
  ;[1 1 1 1 40] Dash
  (set `CharacterMovementComponent.BrakingFriction` 0.0 (`self.CharacterMovement`)))

(event `CameraZoom`
  (`/Engine/EditorBlueprintResources/StandardMacros.DoOnce` false :!label _label_10
    (:`Completed`
      (bind (_direction _time) (`Timeline|ZoomIn` :!via `PlayFromStart`)
        (:`Update`
          (set `SpringArmComponent.TargetArmLength` (`KismetMathLibrary.Lerp` 1900.0 1600.0 _time) (`self.SpringArm`)))
        (:`Finished`
          (goto _label_11 :!via `Reset`))))))

(event `Damage`
  ;[1 1 1] Damage
  (if (> (`self.CurrentHealth`) 0.0)
    (set `self.CurrentHealth` (- (`self.CurrentHealth`) 1.0))
    (if (== (`self.CurrentHealth`) 0.0)
      (`self.Disassemble`))))

(event `CameraZoomOut`
  (`/Engine/EditorBlueprintResources/StandardMacros.DoOnce` false :!label _label_11
    (:`Completed`
      (bind (_direction _time) (`Timeline|Timeline_2` :!via `PlayFromStart`)
        (:`Update`
          (set `SpringArmComponent.TargetArmLength` (`KismetMathLibrary.Lerp` 1600.0 1900.0 _time) (`self.SpringArm`)))
        (:`Finished`
          (goto _label_10 :!via `Reset`))))))

(event `Key|One`
  (params (Key :type "Key Structure"))
  (:`Pressed`
    (`self.Damage`)))

(fn `SetLaserLength`
  (locals (LaserMaxDistance :type "Float (double-precision)" :default 500.0))
  (bind _bulletspawn (`self.BulletSpawn`))
  (bind _returnvalue (`SceneComponent.K2_GetComponentLocation` _bulletspawn))
  (bind (_outhit _returnvalue_2) (`KismetSystemLibrary.LineTraceSingle` _returnvalue (+ _returnvalue (* (`SceneComponent.GetForwardVector` _bulletspawn) 1000.0)) "TraceTypeQuery1"))
  (if _returnvalue_2
    (bind (_bblockinghit _binitialoverlap _time _distance _location _impactpoint _normal _impactnormal _physmat _hitactor) (`GameplayStatics.BreakHitResult` _outhit))
    (bind _output_get (set `local.LaserMaxDistance` _distance))
    (`FXSystemComponent.SetVectorParameter` (`self.LaserSight`) "Beam End" (`KismetMathLibrary.MakeVector` _output_get))
    (if _bblockinghit
      (bind _asbp_assembly_arm (cast `/Game/Blueprints/Class/BP_AssemblyArm` _hitactor)
        (:`then`
          (set `self.ArmHit` true)
          (`/Game/Blueprints/Class/BP_AssemblyArm.AddOutline` _asbp_assembly_arm))
        (:`CastFailed`
          (set `self.ArmHit` false)
          (bind _asbp_destructible (cast `/Game/Blueprints/Class/BP_Destructible` _hitactor)
            (:`then`
              (if (not (`/Game/Blueprints/Class/BP_Destructible.Broken` _asbp_destructible))
                (`/Game/Blueprints/Class/BP_Destructible.AddOutline` _asbp_destructible)
                (set `self.BoxHit` true)))
            (:`CastFailed`
              (set `self.BoxHit` false))))))
    (else
      (set `self.ArmHit` false)
      (set `self.BoxHit` false))))

(fn `UserConstructionScript`)