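; Gas-pipe flame hazard that repeatedly damages the player robot from first contact until it is dead, with no exit check.
; TurnOn ignites it with effects, shake and sound.
; A second box scales in a prompt widget if GameState has the gas wheel, otherwise a hologram wheel.
; With the wheel, TurnOff locks input, mounts and spins the valve, plays a camera cutscene as flames fade, then restores control.
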(event `self.ReceiveBeginPlay`
  (bind _asbp_game_state (cast `/Game/Blueprints/Class/BP_GameState` (`GameplayStatics.GetGameState`)))
  (set `self.As BP Game State` _asbp_game_state)
  (`KismetSystemLibrary.Delay` 2.0)
  (`self.HoloWheelOn`)
  (`KismetSystemLibrary.Delay` 3.0)
  (`self.HoloWheelOff`))

(event `self.Box.OnComponentBeginOverlap`
  (params (OverlappedComponent :type "PrimitiveComponent Object Reference") (OtherActor :type "Actor Object Reference") (OtherComp :type "PrimitiveComponent Object Reference") (OtherBodyIndex :type Integer) (bFromSweep :type Boolean) (SweepResult :type "HitResult Structure (by ref)"))
  (bind _returnvalue (`GameplayStatics.GetPlayerPawn` 0))
  (if (== OtherActor _returnvalue)
    (bind _asbp_robot (cast `/Game/Blueprints/Class/BP_Robot` _returnvalue))
    (if (not (`/Game/Blueprints/Class/BP_Robot.Dead` _asbp_robot)) :!label _label
      (`/Game/Blueprints/Class/BP_Robot.Damage` _asbp_robot)
      (`KismetSystemLibrary.RetriggerableDelay` 0.5)
      (goto _label))))

(event `TurnOff`
  (bind _returnvalue (`GameplayStatics.GetPlayerPawn` 0))
  (bind _returnvalue_2 (`GameplayStatics.GetPlayerController` 0))
  (set `self.PipeOff` true)
  (if (`/Game/Blueprints/Class/BP_GameState.HasGasWheel` (`self.As BP Game State`))
    (`/Engine/EditorBlueprintResources/StandardMacros.DoOnce` false
      (:`Completed`
        (`self.DisableInput` (`GameplayStatics.GetPlayerPawn` 0) (`GameplayStatics.GetPlayerController` 0))
        (`PrimitiveComponent.SetCollisionEnabled` (`self.Box`) "NoCollision")
        (`SceneComponent.SetVisibility` (`self.HoloWheel`) false false)
        (`SceneComponent.SetVisibility` (`self.Wheel`) true false)
        (set `/Game/Blueprints/Class/BP_GameState.HasGasWheel` false (`self.As BP Game State`))
        (`SceneComponent.SetVisibility` (`self.Widget`) false false)
        (bind _asbp_robot (cast `/Game/Blueprints/Class/BP_Robot` (`GameplayStatics.GetPlayerPawn` 0)))
        (`SceneComponent.SetVisibility` (`/Game/Blueprints/Class/BP_Robot.BackItem` _asbp_robot) false false)
        (`|ExecutionSequence`
          (:`then_0`
            (`KismetSystemLibrary.Delay` 1.0)
            (`ActorComponent.Activate` (`self.Valve_Wheel__Squeaky__Turning`) true)
            (bind (_direction _rotate) (`Timeline|Timeline_5` :!via `PlayFromStart`)
              (:`Update`
                (`SceneComponent.K2_SetRelativeRotation` (`self.Wheel`) (`KismetMathLibrary.RLerp` (struct :`Yaw` 90.0) (struct :`Yaw` 90.0 :`Roll` -360.0) _rotate) false false))
              (:`Finished`
                (`ActorComponent.Deactivate` (`self.Valve_Wheel__Squeaky__Turning`)))))
          (:`then_1`
            (`KismetSystemLibrary.Delay` 2.0)
            (bind _returnvalue_3 (`GameplayStatics.GetActorOfClass` "/Game/Blueprints/Class/BP_Camera2.BP_Camera2_C"))
            (`PlayerController.SetViewTargetWithBlend` (`GameplayStatics.GetPlayerController` 0) _returnvalue_3 2.0 "VTBlend_EaseInOut" 2.0 false)
            (`KismetSystemLibrary.Delay` 2.0)
            (bind (_outactor _returnvalue_4) (`LevelSequencePlayer.CreateLevelSequencePlayer` "/Game/Sequences/PipeOff.PipeOff"))
            (`MovieSceneSequencePlayer.Play` _returnvalue_4)
            (`AudioComponent.FadeOut` (`self.GasSound`) 4.0 0.0 "Linear")
            (bind (_direction_2 _rotate_2) (`Timeline|Timeline` :!via `PlayFromStart`)
              (:`Update`
                (`NiagaraComponent.SetVariableFloat` (`self.Flames`) "Life" (`KismetMathLibrary.Lerp` 0.5 0.0 _rotate_2)))
              (:`Finished`
                (`SceneComponent.SetVisibility` (`self.Flames`) false false)
                (`PlayerController.SetViewTargetWithBlend` _returnvalue_2 _returnvalue 2.0 "VTBlend_EaseInOut" 2.0 false)
                (`KismetSystemLibrary.Delay` 2.0)
                (`self.EnableInput` _returnvalue _returnvalue_2)))))))))

(event `TurnOn`
  (bind _returnvalue (`SceneComponent.K2_GetComponentLocation` (`self.Flames`)))
  (`ActorComponent.Activate` (`self.PS_Fire`) true)
  (`GameplayStatics.PlayWorldCameraShake` "/Game/Blueprints/Class/BP_CameraShake.BP_CameraShake_C" _returnvalue 0.0 2000.0)
  (`GameplayStatics.PlaySoundAtLocation` "/Game/Audio/PipeExplode.PipeExplode" _returnvalue (struct) 1.0 1.0 0.0 null null null null)
  (`|ExecutionSequence`
    (:`then_0`
      (`KismetSystemLibrary.Delay` 0.4)
      (`SceneComponent.SetVisibility` (`self.Flames`) true false)
      (bind (_direction _rotate) (`Timeline|Timeline_2` :!via `PlayFromStart`)
        (:`Update`
          (`NiagaraComponent.SetVariableFloat` (`self.Flames`) "Life" (`KismetMathLibrary.Lerp` 0.0 0.5 _rotate)))
        (:`Finished`
          (bind _returnvalue_2 (`GameplayStatics.SpawnSoundAtLocation` "/Game/Audio/GasFlameLoop.GasFlameLoop" _returnvalue (struct) 1.0 1.0 0.0 "/Game/Audio/FurnaceSoundAttenuation.FurnaceSoundAttenuation" null))
          (set `self.GasSound` _returnvalue_2))))
    (:`then_1`
      (`KismetSystemLibrary.Delay` 1.5)
      (bind _returnvalue_3 (`GameplayStatics.SpawnSoundAtLocation` "/Game/Audio/GasFlameLoop.GasFlameLoop" _returnvalue (struct) 1.0 1.0 0.0 null null))
      (`AudioComponent.FadeOut` _returnvalue_3 3.0 0.0 "Linear"))))

(event `self.Box1.OnComponentBeginOverlap`
  (params (OverlappedComponent :type "PrimitiveComponent Object Reference") (OtherActor :type "Actor Object Reference") (OtherComp :type "PrimitiveComponent Object Reference") (OtherBodyIndex :type Integer) (bFromSweep :type Boolean) (SweepResult :type "HitResult Structure (by ref)"))
  (if (== OtherActor (`GameplayStatics.GetPlayerPawn` 0))
    (if (`/Game/Blueprints/Class/BP_GameState.HasGasWheel` (`self.As BP Game State`))
      (`/Engine/EditorBlueprintResources/StandardMacros.DoOnce` false :!label _label_2
        (:`Completed`
          (`self.UIOn`)
          (`KismetSystemLibrary.Delay` 0.2)
          (goto _label_4 :!via `Reset`)))
      (else
        (`/Engine/EditorBlueprintResources/StandardMacros.DoOnce` false :!label _label_3
          (:`Completed`
            (`self.HoloWheelOn`)
            (`KismetSystemLibrary.Delay` 0.2)
            (goto _label_5 :!via `Reset`)))))))

(event `self.Box1.OnComponentEndOverlap`
  (params (OverlappedComponent :type "PrimitiveComponent Object Reference") (OtherActor :type "Actor Object Reference") (OtherComp :type "PrimitiveComponent Object Reference") (OtherBodyIndex :type Integer))
  (if (== OtherActor (`GameplayStatics.GetPlayerPawn` 0))
    (if (`/Game/Blueprints/Class/BP_GameState.HasGasWheel` (`self.As BP Game State`))
      (`/Engine/EditorBlueprintResources/StandardMacros.DoOnce` true :!label _label_4
        (:`Completed`
          (`self.UIOff`)
          (`KismetSystemLibrary.Delay` 0.2)
          (goto _label_2 :!via `Reset`)))
      (else
        (`/Engine/EditorBlueprintResources/StandardMacros.DoOnce` true :!label _label_5
          (:`Completed`
            (`self.HoloWheelOff`)
            (`KismetSystemLibrary.Delay` 0.2)
            (goto _label_3 :!via `Reset`)))))))

(event `UIOn`
  (`/Engine/EditorBlueprintResources/StandardMacros.DoOnce` false :!label _label_6
    (:`Completed`
      (`|ExecutionSequence`
        (:`then_0`
          (bind (_direction _newtrack_0) (`Timeline|Timeline_1` :!via `Stop` :!label _label_7)
            (:`Update`
              (`SceneComponent.SetWorldScale3D` (`self.Widget`) (`KismetMathLibrary.VLerp` (0.5 0.5 0.5) (0.01 0.01 0.01) _newtrack_0)))
            (:`Finished`
              (goto _label_6 :!via `Reset`))))
        (:`then_1`
          (bind (_direction_2 _newtrack_0_2) (`Timeline|Timeline_0` :!via `PlayFromStart` :!label _label_8)
            (:`Update`
              (`SceneComponent.SetWorldScale3D` (`self.Widget`) (`KismetMathLibrary.VLerp` (0.01 0.01 0.01) (0.5 0.5 0.5) _newtrack_0_2)))
            (:`Finished`
              (goto _label_9 :!via `Reset`))))
        (:`then_2`
          (goto _label_9 :!via `Reset`))))))

(event `UIOff`
  (`/Engine/EditorBlueprintResources/StandardMacros.DoOnce` false :!label _label_9
    (:`Completed`
      (`|ExecutionSequence`
        (:`then_0`
          (goto _label_8 :!via `Stop`))
        (:`then_1`
          (goto _label_7 :!via `PlayFromStart`))
        (:`then_2`
          (goto _label_6 :!via `Reset`))))))

(event `HoloWheelOn`
  (`/Engine/EditorBlueprintResources/StandardMacros.DoOnce` false :!label _label_10
    (:`Completed`
      (`|ExecutionSequence`
        (:`then_0`
          (bind (_direction _newtrack_0) (`Timeline|Timeline_4` :!via `Stop` :!label _label_11)
            (:`Update`
              (`SceneComponent.SetWorldScale3D` (`self.HoloWheel`) (`KismetMathLibrary.VLerp` (1.0 1.0 1.0) (0.0 0.0 0.0) _newtrack_0)))
            (:`Finished`
              (goto _label_10 :!via `Reset`))))
        (:`then_1`
          (bind (_direction_2 _newtrack_0_2) (`Timeline|Timeline_3` :!via `PlayFromStart` :!label _label_12)
            (:`Update`
              (`SceneComponent.SetWorldScale3D` (`self.HoloWheel`) (`KismetMathLibrary.VLerp` (0.0 0.0 0.0) (1.0 1.0 1.0) _newtrack_0_2)))
            (:`Finished`
              (goto _label_13 :!via `Reset`))))
        (:`then_2`
          (goto _label_13 :!via `Reset`))))))

(event `HoloWheelOff`
  (`/Engine/EditorBlueprintResources/StandardMacros.DoOnce` false :!label _label_13
    (:`Completed`
      (`|ExecutionSequence`
        (:`then_0`
          (goto _label_12 :!via `Stop`))
        (:`then_1`
          (goto _label_11 :!via `PlayFromStart`))
        (:`then_2`
          (goto _label_10 :!via `Reset`))))))

(fn `UserConstructionScript`)