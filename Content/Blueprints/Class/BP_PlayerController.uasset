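; Player controller that moves the player from the main menu into control of the robot pawn.
; On BeginPlay it adds the robot input mapping, caches the BP_Robot pawn and possesses the BP_MainMenu actor.
; ExitMenu blends the view back to the robot, switches to game-only input, possesses it after the blend, shows a pop-up widget and destroys the menu actor.
; Respawn re-caches the robot; cursor-aim and crosshair logic is disconnected.
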(event `self.ReceiveBeginPlay`
  (bind _returnvalue (subsystem `EnhancedInputLocalPlayerSubsystem`))
  (`/Engine/EditorBlueprintResources/StandardMacros.IsValid` _returnvalue
    (:`Is Valid`
      (`EnhancedInputSubsystemInterface.AddMappingContext` _returnvalue "/Game/Misc/Inputs/IMC_Robot.IMC_Robot" 0 (struct))
      (bind _asbp_robot (cast `/Game/Blueprints/Class/BP_Robot` (`GameplayStatics.GetPlayerPawn` 0)))
      (set `self.As Robot BP` _asbp_robot)
      (bind _returnvalue_2 (`GameplayStatics.GetActorOfClass` "/Game/Blueprints/Class/BP_MainMenu.BP_MainMenu_C"))
      (`self.Possess` (`GameplayStatics.GetPlayerController` 0) _returnvalue_2))))

(event `ExitMenu`
  (bind _returnvalue (`GameplayStatics.GetPlayerController` 0))
  (bind _as_robot_bp (`self.As Robot BP`))
  (`self.SetViewTargetWithBlend` (`GameplayStatics.GetPlayerController` 0) _as_robot_bp 3.0 "VTBlend_Linear" 0.0 false)
  (set `PlayerController.bShowMouseCursor` false _returnvalue)
  (`WidgetBlueprintLibrary.SetInputMode_GameOnly` _returnvalue)
  (`KismetSystemLibrary.Delay` 3.0)
  (`self.Possess` (`GameplayStatics.GetPlayerController` 0) _as_robot_bp)
  (bind _returnvalue_2 (`|CreateWidget` "/Game/Blueprints/UI/BP_PopUp_Widget.BP_PopUp_Widget_C"))
  (bind _output_get (set `self.PopUpWidget` _returnvalue_2))
  (`UserWidget.AddToViewport` _output_get 0)
  (`/Game/Blueprints/UI/BP_PopUp_Widget.Move` _output_get)
  (`self.K2_DestroyActor` (stale `self.ReceiveBeginPlay` _returnvalue_2)))

(event `Respawn`
  (bind _asbp_robot (cast `/Game/Blueprints/Class/BP_Robot` (`GameplayStatics.GetPlayerPawn` 0)))
  (set `self.As Robot BP` _asbp_robot))

(event `self.ReceiveTick`
  (params (DeltaSeconds :type "Float (single-precision)")))

(fn `UserConstructionScript`)