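; Security console that shows whether the system is locked and lets a lockdown be cleared.
; While locked, the player entering its box scales the UI widget up through timelines, and leaving scales it down.
; LockDown sets the locked screen material and re-arms ResetSystem.
; ResetSystem opens every security door, ends lockdown on all cameras and laser bots, switches to the open screen and hides the UI.
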(event `UIOn`
  (if (`self.SystemLocked`)
    (`/Engine/EditorBlueprintResources/StandardMacros.DoOnce` false :!label _label
      (:`Completed`
        (`|ExecutionSequence`
          (:`then_0`
            (bind (_direction _newtrack_0) (`Timeline|Timeline_0` :!via `Stop` :!label _label_2)
              (:`Update`
                (`SceneComponent.SetWorldScale3D` (`self.Widget`) (`KismetMathLibrary.VLerp` (1.0 1.0 1.0) (0.01 0.01 0.01) _newtrack_0)))
              (:`Finished`
                (goto _label :!via `Reset`))))
          (:`then_1`
            (bind (_direction_2 _newtrack_0_2) (`Timeline|Timeline` :!via `PlayFromStart` :!label _label_3)
              (:`Update`
                (`SceneComponent.SetWorldScale3D` (`self.Widget`) (`KismetMathLibrary.VLerp` (0.01 0.01 0.01) (1.0 1.0 1.0) _newtrack_0_2)))
              (:`Finished`
                (goto _label_4 :!via `Reset`))))
          (:`then_2`
            (goto _label_4 :!via `Reset`)))))))

(event `UIOff`
  (`/Engine/EditorBlueprintResources/StandardMacros.DoOnce` false :!label _label_4
    (:`Completed`
      (`|ExecutionSequence`
        (:`then_0`
          (goto _label_3 :!via `Stop`))
        (:`then_1`
          (goto _label_2 :!via `PlayFromStart`))
        (:`then_2`
          (goto _label :!via `Reset`))))))

(event `self.Box.OnComponentBeginOverlap`
  (params (OverlappedComponent :type "PrimitiveComponent Object Reference") (OtherActor :type "Actor Object Reference") (OtherComp :type "PrimitiveComponent Object Reference") (OtherBodyIndex :type Integer) (bFromSweep :type Boolean) (SweepResult :type "HitResult Structure (by ref)"))
  (if (== OtherActor (`GameplayStatics.GetPlayerPawn` 0))
    (`self.UIOn`)))

(event `self.Box.OnComponentEndOverlap`
  (params (OverlappedComponent :type "PrimitiveComponent Object Reference") (OtherActor :type "Actor Object Reference") (OtherComp :type "PrimitiveComponent Object Reference") (OtherBodyIndex :type Integer))
  (if (== OtherActor (`GameplayStatics.GetPlayerPawn` 0))
    (`self.UIOff`)))

(event `LockDown`
  (if (not (`self.SystemLocked`))
    (`PrimitiveComponent.SetMaterial` (`self.Screen`) 1 "/Game/TEMP/M_Screen_Inst.M_Screen_Inst")
    (set `self.SystemLocked` true)
    (goto _label_5 :!via `Reset`)))

(event `ResetSystem`
  (if (`self.SystemLocked`)
    (`/Engine/EditorBlueprintResources/StandardMacros.DoOnce` false :!label _label_5
      (:`Completed`
        (`PrimitiveComponent.SetMaterial` (`self.Screen`) 1 "/Game/TEMP/M_Screen_Open.M_Screen_Open")
        (bind _outactors (`GameplayStatics.GetAllActorsOfClass` "/Game/Blueprints/Class/BP_SecurityDoor.BP_SecurityDoor_C"))
        (for _array_element _outactors
          (`/Game/Blueprints/Class/BP_SecurityDoor.OpenDoor` _array_element))
        (bind _outactors_2 (`GameplayStatics.GetAllActorsOfClass` "/Game/Blueprints/Class/BP_SecurityCamera.BP_SecurityCamera_C"))
        (for _array_element_2 _outactors_2
          (`/Game/Blueprints/Class/BP_SecurityCamera.LockdownEnd` _array_element_2))
        (bind _outactors_3 (`GameplayStatics.GetAllActorsOfClass` "/Game/Blueprints/Class/BP_LaserBot.BP_LaserBot_C"))
        (for _array_element_3 _outactors_3
          (set `/Game/Blueprints/Class/BP_LaserBot.Lockdown` false _array_element_3))
        (set `self.SystemLocked` false)
        (`self.UIOff`)
        (goto _label :!via `Reset`)))))

(fn `UserConstructionScript`
  (if (`self.SystemLocked`)
    (`PrimitiveComponent.SetMaterial` (`self.Screen`) 1 "/Game/TEMP/M_Screen_Inst.M_Screen_Inst")
    (else
      (`PrimitiveComponent.SetMaterial` (`self.Screen`) 1 "/Game/TEMP/M_Screen_Open.M_Screen_Open"))))