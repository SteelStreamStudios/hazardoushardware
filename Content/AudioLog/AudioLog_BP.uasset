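; AudioLog_BP is a collectible audio log with a pickup prompt plane.
; Sphere overlap with the player pawn drives two timelines that lerp the plane's scale up on entry and down to zero on exit, each stopping the other.
; The PickUp event uses AudioLogNum to play one of two 2D sounds, set the matching picked-up flag on GameState_BP, then destroy the actor.
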(event `self.ReceiveBeginPlay`
  (bind _asgame_state_bp (cast `/Game/PlayerCharacter/Blueprints/GameState_BP` (`GameplayStatics.GetGameState`)))
  (set `self.GameState` _asgame_state_bp))

(event `self.Sphere.OnComponentBeginOverlap`
  (params (OverlappedComponent :type "PrimitiveComponent Object Reference") (OtherActor :type "Actor Object Reference") (OtherComp :type "PrimitiveComponent Object Reference") (OtherBodyIndex :type Integer) (bFromSweep :type Boolean) (SweepResult :type "HitResult Structure (by ref)"))
  ;[1 1 1] "Press E" Prompt Active
  (if (== OtherActor (`GameplayStatics.GetPlayerPawn` 0))
    (`|ExecutionSequence`
      (:`then_0`
        (bind (_direction _time) (`Timeline|Timeline` :!via `PlayFromStart` :!label _label)
          (:`Update`
            (`SceneComponent.SetWorldScale3D` (`self.Plane`) (`KismetMathLibrary.VLerp` (`SceneComponent.K2_GetComponentScale` (`self.Plane`)) (2.8 2.8 2.8) _time)))))
      (:`then_1`
        ;[1 1 1] "Press E" Prompt Deactive
        (bind (_direction_2 _time_2) (`Timeline|Timeline_0` :!via `Stop` :!label _label_2)
          (:`Update`
            (`SceneComponent.SetWorldScale3D` (`self.Plane`) (`KismetMathLibrary.VLerp` (`SceneComponent.K2_GetComponentScale` (`self.Plane`)) (0.0 0.0 0.0) _time_2))))))))

(event `self.Sphere.OnComponentEndOverlap`
  (params (OverlappedComponent :type "PrimitiveComponent Object Reference") (OtherActor :type "Actor Object Reference") (OtherComp :type "PrimitiveComponent Object Reference") (OtherBodyIndex :type Integer))
  ;[1 1 1] "Press E" Prompt Deactive
  (if (== OtherActor (`GameplayStatics.GetPlayerPawn` 0))
    (`|ExecutionSequence`
      (:`then_0`
        (goto _label :!via `Stop`))
      (:`then_1`
        (goto _label_2 :!via `PlayFromStart`)))))

(event `/Game/AudioLog/PickUp_Interface.PickUp`
  (if (== (`self.AudioLogNum`) 1)
    (`GameplayStatics.PlaySound2D` "/Game/AudioLog/Sounds/Halo_Infinite__All_Campaign_Audio_Logs.Halo_Infinite__All_Campaign_Audio_Logs" 1.0 1.0 0.0 null null)
    (set `/Game/PlayerCharacter/Blueprints/GameState_BP.AudioLog1PickedUp` true (`self.GameState`))
    (`self.K2_DestroyActor`)
    (elif (== (`self.AudioLogNum`) 2)
      (`GameplayStatics.PlaySound2D` "/Engine/VREditor/Sounds/UI/Camera_Shutter.Camera_Shutter" 1.0 1.0 0.0 null null)
      (set `/Game/PlayerCharacter/Blueprints/GameState_BP.AudioLog2PickedUp` true (`self.GameState`))
      (`self.K2_DestroyActor`))))

(fn `UserConstructionScript`)