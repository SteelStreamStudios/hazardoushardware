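; Player controller for the robot character that sets up Enhanced Input, the follow camera and a mouse-driven crosshair.
; On BeginPlay it adds the robot mapping context, hides the cursor, creates the crosshair widget and makes a spawned camera actor the view target.
; While the robot lives, Tick moves the camera to the robot's arrow component.
; With a gun equipped, it also sends the cursor hit location as a look-at message and moves the crosshair to the mouse.
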(event `self.ReceiveBeginPlay`
  (bind _returnvalue (subsystem `EnhancedInputLocalPlayerSubsystem`))
  (`/Engine/EditorBlueprintResources/StandardMacros.IsValid` _returnvalue
    (:`Is Valid`
      (`EnhancedInputSubsystemInterface.AddMappingContext` _returnvalue "/Game/PlayerCharacter/Inputs/IMC_Robot.IMC_Robot" 0 (struct))
      (set `self.bShowMouseCursor` false)
      (bind _asrobot_bp (cast `/Game/PlayerCharacter/Blueprints/Robot_BP` (`GameplayStatics.GetPlayerPawn` 0)))
      (bind _output_get (set `self.As Robot BP` _asrobot_bp))
      (bind _output_get_2 (set `self.PlayerRef` (`GameplayStatics.GetPlayerController` 0)))
      (bind _returnvalue_2 (`|CreateWidget` "/Game/UI/Target/Crossair_Widget.Crossair_Widget_C" _output_get_2))
      (set `self.CrossairWidget` _returnvalue_2)
      (bind _returnvalue_3 (`|SpawnActorFromClass` "/Game/PlayerCharacter/Blueprints/PlayerCamera_BP.PlayerCamera_BP_C" (`SceneComponent.K2_GetComponentToWorld` (`/Game/PlayerCharacter/Blueprints/Robot_BP.Arrow1` _output_get)) "Undefined" "MultiplyWithRoot" null null))
      (bind _output_get_3 (set `self.PlayerCam` _returnvalue_3))
      (`self.SetViewTargetWithBlend` _output_get_3))))

(event `AddCrossairs`
  (`UserWidget.AddToViewport` (`self.CrossairWidget`) 0))

(event `RemoveCrossairs`
  (`Widget.RemoveFromParent` (`self.CrossairWidget`)))

(event `self.ReceiveTick`
  (params (DeltaSeconds :type "Float (single-precision)"))
  (bind (_locationx _locationy) (`self.GetMousePosition`))
  (if (not (`/Game/PlayerCharacter/Blueprints/Robot_BP.Dead` (`self.As Robot BP`)))
    (`SceneComponent.K2_SetWorldLocation` (`/Game/PlayerCharacter/Blueprints/PlayerCamera_BP.DefaultSceneRoot` (`self.PlayerCam`)) (`SceneComponent.K2_GetComponentLocation` (`/Game/PlayerCharacter/Blueprints/Robot_BP.Arrow1` (`self.As Robot BP`))) false false)
    (if (`/Game/PlayerCharacter/Blueprints/Robot_BP.GunEquipped` (`self.As Robot BP`))
      (message `/Game/PlayerCharacter/Blueprints/RobotInterface_BP.LookAt` (`GameplayStatics.GetPlayerPawn` 0) (`.Location` (`GameplayStatics.BreakHitResult` (`self.GetHitResultUnderCursorByChannel` "TraceTypeQuery1"))))
      (`UserWidget.SetPositionInViewport` (`self.CrossairWidget`) (`KismetMathLibrary.MakeVector2D` _locationx _locationy) true))))

(fn `UserConstructionScript`)