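; Test electrified floor hazard that switches on and off every ten seconds, starting after an initial delay.
; A looping delay calls FloorSwitch, which flips FloorOn and recolors a dynamic material: green when on, red when off.
; The construction script creates that material and sets its color from the initial state.
; Box begin-overlap damages the player's BP_Robot only if the floor is on at entry.
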(event `self.ReceiveBeginPlay`
  (`KismetSystemLibrary.Delay` 10.0)
  (`self.FloorSwitch` :!label _label)
  (`KismetSystemLibrary.RetriggerableDelay` 10.0)
  (goto _label))

(event `self.Box.OnComponentBeginOverlap`
  (params (OverlappedComponent :type "PrimitiveComponent Object Reference") (OtherActor :type "Actor Object Reference") (OtherComp :type "PrimitiveComponent Object Reference") (OtherBodyIndex :type Integer) (bFromSweep :type Boolean) (SweepResult :type "HitResult Structure (by ref)"))
  (bind _returnvalue (`GameplayStatics.GetPlayerPawn` 0))
  ;[1 1 1] Electrify Player
  (if (== OtherActor _returnvalue)
    (if (`self.FloorOn`)
      (bind _asbp_robot (cast `/Game/Blueprints/Class/BP_Robot` _returnvalue))
      (`/Game/Blueprints/Class/BP_Robot.Damage` _asbp_robot))))

(event `FloorSwitch`
  (if (`self.FloorOn`)
    (`MaterialInstanceDynamic.SetVectorParameterValue` (`self.Mat`) "Color" (struct :`R` 0.572917 :`B` 0.008895 :`A` 1.0))
    (set `self.FloorOn` false)
    (else
      (`MaterialInstanceDynamic.SetVectorParameterValue` (`self.Mat`) "Color" (struct :`G` 0.572917 :`B` 0.029321 :`A` 1.0))
      (set `self.FloorOn` true))))

(fn `UserConstructionScript`
  (bind _cube (`self.Cube`))
  (bind _returnvalue (`PrimitiveComponent.CreateDynamicMaterialInstance` _cube 0 (`PrimitiveComponent.GetMaterial` _cube 0) "None"))
  (bind _output_get (set `self.Mat` _returnvalue))
  (if (`self.FloorOn`)
    (`MaterialInstanceDynamic.SetVectorParameterValue` _output_get "Color" (struct :`G` 0.572917 :`B` 0.029321 :`A` 1.0))
    (else
      (`MaterialInstanceDynamic.SetVectorParameterValue` _output_get "Color" (struct :`R` 0.572917 :`B` 0.008895 :`A` 1.0)))))