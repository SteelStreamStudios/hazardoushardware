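; ElectricalSwitch_BP is an electrical switch the player robot can interact with while inside its trigger box.
; Box overlap sets CanInteract on Robot_BP and calls UIOn or UIOff.
; Two timelines lerp a plane's world scale up or down and toggle two Niagara components' visibility.
; A pair of DoOnce gates, each reset when the opposite timeline finishes, keeps the show and hide animations from retriggering.
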(event `self.Box.OnComponentBeginOverlap`
  (params (OverlappedComponent :type "PrimitiveComponent Object Reference") (OtherActor :type "Actor Object Reference") (OtherComp :type "PrimitiveComponent Object Reference") (OtherBodyIndex :type Integer) (bFromSweep :type Boolean) (SweepResult :type "HitResult Structure (by ref)"))
  (bind _returnvalue (`GameplayStatics.GetPlayerPawn` 0))
  (if (== OtherActor _returnvalue)
    (bind _asrobot_bp (cast `/Game/PlayerCharacter/Blueprints/Robot_BP` _returnvalue))
    (set `/Game/PlayerCharacter/Blueprints/Robot_BP.CanInteract` true _asrobot_bp)
    (`self.UIOn`)))

(event `self.Box.OnComponentEndOverlap`
  (params (OverlappedComponent :type "PrimitiveComponent Object Reference") (OtherActor :type "Actor Object Reference") (OtherComp :type "PrimitiveComponent Object Reference") (OtherBodyIndex :type Integer))
  (bind _returnvalue (`GameplayStatics.GetPlayerPawn` 0))
  (if (== OtherActor _returnvalue)
    (bind _asrobot_bp (cast `/Game/PlayerCharacter/Blueprints/Robot_BP` _returnvalue))
    (set `/Game/PlayerCharacter/Blueprints/Robot_BP.CanInteract` false _asrobot_bp)
    (`self.UIOff`)))

(event `UIOn`
  (`/Engine/EditorBlueprintResources/StandardMacros.DoOnce` false :!label _label
    (:`Completed`
      (bind (_direction _newtrack_0) (`Timeline|On` :!via `PlayFromStart`)
        (:`Update`
          (`SceneComponent.SetWorldScale3D` (`self.Plane`) (`KismetMathLibrary.VLerp` (`SceneComponent.K2_GetComponentScale` (`self.Plane`)) (2.0 2.0 2.0) _newtrack_0))
          (`SceneComponent.SetVisibility` (`self.Niagara`) true false)
          (`SceneComponent.SetVisibility` (`self.Niagara1`) true false))
        (:`Finished`
          (goto _label_2 :!via `Reset`))))))

(event `UIOff`
  (`/Engine/EditorBlueprintResources/StandardMacros.DoOnce` false :!label _label_2
    (:`Completed`
      (bind (_direction _newtrack_0) (`Timeline|Timeline` :!via `PlayFromStart`)
        (:`Update`
          (`SceneComponent.SetWorldScale3D` (`self.Plane`) (`KismetMathLibrary.VLerp` (`SceneComponent.K2_GetComponentScale` (`self.Plane`)) (0.0 0.0 0.0) _newtrack_0))
          (`SceneComponent.SetVisibility` (`self.Niagara`) false false)
          (`SceneComponent.SetVisibility` (`self.Niagara1`) false false))
        (:`Finished`
          (goto _label :!via `Reset`))))))

(fn `UserConstructionScript`)