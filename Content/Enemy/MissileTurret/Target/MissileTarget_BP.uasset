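; Missile turret target marker that runs a timing check for blocking an incoming missile.
; StartTarget gives the Goal component a random scale, while a timeline eases the Target component toward unit scale and Tick records its current size.
; StopMissile sets BlockMissile and destroys the actor if Target's X scale is within a narrow window around Goal's.
; If the timeline finishes first, it spawns an emitter at Target and destroys the actor.
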(event `self.ReceiveTick`
  (params (DeltaSeconds :type "Float (single-precision)"))
  (if (`self.Targeting`)
    (set `self.TargetSize` (`SceneComponent.K2_GetComponentScale` (`self.Target`)))))

(event `StartTarget`
  (bind _returnvalue (`KismetMathLibrary.RandomFloatInRange` 1.3 3.0))
  ;[1 1 1] Start Targeting
  (`|ExecutionSequence`
    (:`then_0`
      (set `self.Targeting` true)
      (bind (_direction _newtrack_0) (`Timeline|Timeline` :!via `PlayFromStart`)
        (:`Update`
          (`SceneComponent.SetWorldScale3D` (`self.Target`) (`KismetMathLibrary.VLerp` (`SceneComponent.K2_GetComponentScale` (`self.Target`)) (1.0 1.0 1.0) _newtrack_0)))
        (:`Finished`
          (set `self.Targeting` false)
          (`GameplayStatics.SpawnEmitterAtLocation` null (`SceneComponent.K2_GetComponentLocation` (`self.Target`)) (struct) (6.0 6.0 6.0))
          (`KismetSystemLibrary.Delay` 0.1)
          (`self.K2_DestroyActor`))))
    (:`then_1`
      (`SceneComponent.SetWorldScale3D` (`self.Goal`) (`KismetMathLibrary.MakeVector` _returnvalue _returnvalue _returnvalue))
      (set `self.GoalSize` (`SceneComponent.K2_GetComponentScale` (`self.Goal`))))))

(event `StopMissile`
  (bind _targetsize_x (`KismetMathLibrary.BreakVector` (`self.TargetSize`)))
  (bind _goalsize_x (`KismetMathLibrary.BreakVector` (`self.GoalSize`)))
  (bind _goalsize_x_2 (`KismetMathLibrary.BreakVector` (`self.GoalSize`)))
  ;[1 1 1] Stop Missile
  (if (`KismetMathLibrary.InRange_FloatFloat` _targetsize_x (+ _goalsize_x_2 -0.3) (+ _goalsize_x 0.1))
    (set `self.BlockMissile` true)
    (`self.K2_DestroyActor`)
    (else
      (set `self.BlockMissile` false))))

(fn `UserConstructionScript`)