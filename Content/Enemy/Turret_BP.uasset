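; Enemy turret Blueprint, an early stub that switches between Scanning and Attacking behavior on Tick based on TurretState.
; Scanning reads the component-space yaw of the PoseableMesh spine bone and updates a RotateRight flag to reverse sweep direction at symmetric limits.
; The bone rotation is never applied, Attack is empty, and nothing here changes TurretState.
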(event `self.ReceiveTick`
  (params (DeltaSeconds :type "Float (single-precision)"))
  (switch `/Game/Enemy/TurretState_Enum` (`self.TurretState`)
    (:`NewEnumerator0`
      (`self.RotateTurret`))
    (:`NewEnumerator1`
      (`self.Attack`))))

(event `RotateTurret`
  (bind _returnvalue (`PoseableMeshComponent.GetBoneRotationByName` (`self.PoseableMesh`) "Spine02_JNT" "ComponentSpace"))
  (bind _yaw (.yaw _returnvalue))
  (set `self.RotateRight` (or (and (< _yaw 70.0) (`self.RotateRight`)) (and (< _yaw -70.0) (not (`self.RotateRight`))))))

(event `Attack`)

(fn `UserConstructionScript`)